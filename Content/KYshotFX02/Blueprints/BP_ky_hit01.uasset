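; BP_ky_hit01 is a hit effect actor that plays a particle system, with a configurable color and optional looping.
; The construction script passes the Color variable into the particle system's "color" vector parameter.
; On BeginPlay it activates the particle system, waits two seconds, then either re-activates it while IsLoop is set or destroys itself.
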(event EventBeginPlay
  ;[1 1 1] fx activate
  (Components|Activation|Activate (Variables|Default|GetParticleSystem) (Variables|Default|GetisReset) :!label _label)
  ;[1 1 1] loop control
  (Utilities|FlowControl|Delay 2.0)
  (if (Variables|Default|GetisLoop)
    (goto _label)
    (else
      ;[1 1 1] destroy
      (Actor|DestroyActor))))

(event Collision|EventActorBeginOverlap
  (params (OtherActor :type Actor%20Object%20Reference)))

(event EventTick
  (params (DeltaSeconds :type Float%20%28single-precision%29)))

(fn ConstructionScript
  ;[1 1 1] color control
  (Effects|Components|ParticleSystem|SetVectorParameter (Variables|Default|GetParticleSystem) "color" (Math|Conversions|ToVector(LinearColor) (Variables|Components|Getcolor))))