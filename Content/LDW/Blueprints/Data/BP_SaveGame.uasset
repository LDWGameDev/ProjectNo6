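; Save game object that holds player progress: total played time, death count, dialogue index and mission index.
; AddToTotalPlayedTime adds the seconds elapsed since LastStartedPlayTime, ignoring negative durations, and prints the session duration as debug output.
; It neither updates that start timestamp nor saves.
; ResetSaveGame restores the progress fields to their defaults and immediately writes the object to the given slot.
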(event Custom|ResetSaveGame
  (params (SlotName :type String))
  ;[1 1 1] Reset Save Game
  (Variables|Default|SetTotalPlayedTime 0.0)
  (Variables|Default|SetTotalDeathTimes 0)
  (Variables|Default|SetDialogueIndex -1)
  (Variables|Default|SetMissionIndex -1)
  (SaveGame|SaveGametoSlot self SlotName))

(event Custom|AddToTotalPlayedTime
  (bind _returnvalue (Math|DateTime|Now))
  (bind _laststartedplaytime (Variables|Default|GetLastStartedPlayTime))
  (bind _outdurationinseconds (Class|CustomFunctionLibrary|GetDurationinSecondsBetween2DateTime _laststartedplaytime _returnvalue))
  ;[1 1 1] Add To Total Played Time
  (Variables|Default|SetTotalPlayedTime (+ (Variables|Default|GetTotalPlayedTime) (Math|Float|SelectFloat _outdurationinseconds 0.0 (> _outdurationinseconds 0.0))))
  (Development|PrintString (Utilities|GetOuterObject self) (Utilities|String|Append "New played time" (Utilities|String|ToString(Float) _outdurationinseconds))))