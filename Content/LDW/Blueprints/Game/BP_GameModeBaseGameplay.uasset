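; Gameplay game mode Blueprint that holds KE-prefixed debug events for manipulating a play session.
; Kill All Enemies force-kills every BP_EnemyBase actor, and Kill Player force-kills the human player character.
; The Restart, Trigger Temple Selection and Generate Objectives events are empty.
; Their apparent logic (player-start respawn, controller temple selection, game instance floor objectives) sits disconnected and never runs.
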(event Custom|KERestart
  ;[1 1 1] KE Restart
)

(event Custom|KETriggerTempleSelection
  ;[1 1 1] KE Trigger Temple Selection
)

(event Custom|KEGenerateObjectives
  ;[1 1 1] KE Generate Objectives
)

(event Custom|KE_KillAllEnemies
  ;[1 1 1] KE Kill All Enemies
  (bind _outactors (Actor|GetAllActorsOfClass "/Game/LDW/Blueprints/Characters/Enemies/BP_EnemyBase.BP_EnemyBase_C"))
  (for _array_element _outactors
    (Class|CharacterEnemyBase|ForceonDied _array_element)))

(event Custom|KE_KillPlayer
  ;[1 1 1] KE Kill Player
  (bind _returnvalue (Actor|GetActorOfClass "/Game/LDW/Blueprints/Characters/Player/BP_CharacterPlayerHuman.BP_CharacterPlayerHuman_C"))
  (Class|CharacterPlayerBase|ForceDie _returnvalue))

(fn ConstructionScript)