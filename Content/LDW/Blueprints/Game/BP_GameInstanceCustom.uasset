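; Custom Game Instance that carries run-wide state and services for a temple-floor game: settings, music, missions, dialogue and saving.
; It extends parent logic for floors, objectives and enemy deaths, forwarding results to the gameplay controller's widgets and the player's notifications.
; Two persistent 2D audio components swap combat and non-combat music, with volumes set through sound mix class overrides.
; Shutdown saves play time, and the halfway floor triggers a dialogue.
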(event Custom|SetSaveGame
  (params (SaveGame :type BP%20Save%20Game%20Object%20Reference) (SaveSlot :type String))
  ;[1 1 1] SetSaveGame
  (Variables|Default|SetCurrentSaveGame SaveGame)
  (Variables|Default|SetCurrentSaveSlot SaveSlot))

(event Custom|PlayBGMusic
  (params (bIsCombatBGM :type Boolean))
  ;[1 1 1] Play BGM
  (if (and (Utilities|IsValid (Variables|Default|GetNonCombatBGM)) (Utilities|IsValid (Variables|Default|GetCombatBGM)))
    (if bIsCombatBGM
      (Audio|Components|Audio|Stop (Variables|Default|GetNonCombatBGM))
      (Audio|Components|Audio|Play (Variables|Default|GetCombatBGM) 0.0)
      (else
        (Audio|Components|Audio|Stop (Variables|Default|GetCombatBGM))
        (Audio|Components|Audio|Play (Variables|Default|GetNonCombatBGM) 0.0)))))

(event Custom|GrantPlayerNewMission
  (params (MissionClass :type BP%20Mission%20Base%20Class%20Reference))
  ;[1 1 1] Grant Player New Mission
  (bind _returnvalue (Game|ConstructObjectfromClass MissionClass))
  (Default|OnStarted _returnvalue)
  (Utilities|Array|Add (Variables|Default|GetOnGoingMissions) _returnvalue)
  (bind _asbp_player_controller_gameplay (Utilities|Casting|CastToBP_PlayerControllerGameplay (Game|GetPlayerController 0)))
  (Default|AddNewonGoingMission (Variables|/Game/LDW/Blueprints/Widgets/WBP_PersistentGameplay.WBP_PersistentGameplay_C|GetWBP_PersistentMissionsContainer (Variables|/Game/LDW/Blueprints/Characters/Player/BP_PlayerControllerGameplay.BP_PlayerControllerGameplay_C|GetPersistentGameplayWBP _asbp_player_controller_gameplay)) _returnvalue))

(event Custom|RemoveOnGoingMission
  (params (MissionToRemove :type BP%20Mission%20Base%20Object%20Reference))
  ;[1 1 1] Remove On Going Mission
  (Utilities|Array|RemoveItem (Variables|Default|GetOnGoingMissions) MissionToRemove))

(event Custom|StartNewDialogue
  (params (DialogueClass :type BP%20Dialogue%20Base%20Class%20Reference))
  ;[1 1 1] Start New Dialogue
  (if (and (Utilities|IsValidClass DialogueClass) (not (Utilities|IsValid (Variables|Default|GetCurrentDialogue))))
    (bind _returnvalue (Game|ConstructObjectfromClass DialogueClass))
    (bind _output_get (Variables|Default|SetCurrentDialogue _returnvalue))
    (Class|MissionBase|OnStarted _output_get)))

(event Custom|ResetToStartLevel
  ;[1 1 1] Reset To Start Level
  (bind _asbp_player_controller_gameplay (Utilities|Casting|CastToBP_PlayerControllerGameplay (Game|GetPlayerController 0)))
  (Default|TransitionintoBlack (Variables|/Game/LDW/Blueprints/Characters/Player/BP_PlayerControllerGameplay.BP_PlayerControllerGameplay_C|GetTransitionWBP _asbp_player_controller_gameplay))
  (Utilities|FlowControl|Delay 0.3)
  (Game|OpenLevel(byName) "StartLevel"))

(event EventInit
  ;[1 1 1] Init
  (|CallParentFunction)
  (Utilities|FlowControl|Sequence
    (:then_2
      (Utilities|FlowControl|Delay 1.0)
      (bind _returnvalue (Audio|CreateSound2D "/Game/LDW/Assets/Sounds/SCue_BGMNonCombat.SCue_BGMNonCombat" 1.0 1.0 0.0 0 true false))
      (Variables|Default|SetNonCombatBGM _returnvalue)
      (bind _returnvalue_2 (Audio|CreateSound2D "/Game/LDW/Assets/Sounds/SCue_CombatBGM.SCue_CombatBGM" 1.0 1.0 0.0 0 true false))
      (Variables|Default|SetCombatBGM _returnvalue_2))))

(event EventApplyAudioSettings
  ;[1 1 1] Apply Audio Settings
  (bind _returnvalue (Class|CustomFunctionLibrary|GetCustomGameUserSettings))
  (Utilities|IsValid _returnvalue
    (:Is%20Valid
      (Audio|SetSoundMixClassOverride "/Game/LDW/Blueprints/Sounds/SMix_GameplayMix.SMix_GameplayMix" "/Game/LDW/Blueprints/Sounds/SC_Master.SC_Master" (/ (Math|Conversions|ToFloat(Integer) (Class|CustomGameUserSettings|GetMasterVolume _returnvalue)) 1e+02) 1.0 0.0 true)
      (Audio|SetSoundMixClassOverride "/Game/LDW/Blueprints/Sounds/SMix_GameplayMix.SMix_GameplayMix" "/Game/LDW/Blueprints/Sounds/SC_BGMusic.SC_BGMusic" (/ (Math|Conversions|ToFloat(Integer) (Class|CustomGameUserSettings|GetMusicVolume _returnvalue)) 1e+02) 1.0 0.0 true)
      (Audio|SetSoundMixClassOverride "/Game/LDW/Blueprints/Sounds/SMix_GameplayMix.SMix_GameplayMix" "/Game/LDW/Blueprints/Sounds/SC_Effect.SC_Effect" (/ (Math|Conversions|ToFloat(Integer) (Class|CustomGameUserSettings|GetEffectVolume _returnvalue)) 1e+02) 1.0 0.0 true)
      (Class|GameUserSettings|ApplySettings _returnvalue true))))

(event EventOnEnemyDied
  (params (DeathEnemy :type Character%20Enemy%20Base%20Object%20Reference))
  ;[1 1 1] On Enemy Died
  (|CallParentFunction DeathEnemy)
  (Utilities|IsValid DeathEnemy
    (:Is%20Valid
      (bind _asbp_character_player_human (Utilities|Casting|CastToBP_CharacterPlayerHuman (Game|Player|GetPlayerPawn 0)))
      (Default|NotifywithOverHeadNotification _asbp_character_player_human "Kill +1" 1)
      (Default|CallOnEnemyDiedDelegate (Utilities|GetClass DeathEnemy)))))

(event EventHandleonCurrentLevelStreamingShown
  ;[1 1 1] Handle On Current Level Streaming Shown
  (|CallParentFunction)
  (Default|CallOnStreamLevelLoaded)
  (if (== (Variables|Default|GetFloorIndexCount) 2)
    (Utilities|FlowControl|Delay 1.0)
    (CallFunction|StartNewDialogue "/Game/LDW/Blueprints/Mission/BP_DHalfWayNotification.BP_DHalfWayNotification_C")))

(event EventInitSoundMix
  ;[1 1 1] Init Sound Mix
  (|CallParentFunction)
  (Class|GameplayStatics|SetBaseSoundMix "/Game/LDW/Blueprints/Sounds/SMix_BaseMix.SMix_BaseMix")
  (Audio|PushSoundMixModifier "/Game/LDW/Blueprints/Sounds/SMix_GameplayMix.SMix_GameplayMix"))

(event EventApplyGraphicsSettings
  ;[1 1 1] Apply Graphics Settings
  (|CallParentFunction))

(event EventGenerateFloorObjectives
  ;[1 1 1] Generate Floor Objectives
  (|CallParentFunction)
  (bind _asbp_player_controller_gameplay (Utilities|Casting|CastToBP_PlayerControllerGameplay (Game|GetPlayerController 0)))
  (Default|CreateObjectiveWigets _asbp_player_controller_gameplay))

(event EventResetCurrentFloorIndex
  ;[1 1 1] Reset Current Floor Index
  (|CallParentFunction))

(event EventHandleCompletedObjective
  (params (ObjectiveIndex :type Integer) (FloorIndex :type Integer) (ObjectiveType :type EFloorObjectiveType%20Enum :default "Empty"))
  ;[1 1 1] Handle Completed Objective
)

(event EventOnLoadedNewFloor
  (bind _floorindexcount (Variables|Default|GetFloorIndexCount))
  ;[1 1 1] On Loaded New Floor
  (bind _asbp_player_controller_gameplay (Utilities|Casting|CastToBP_PlayerControllerGameplay (Game|GetPlayerController 0)))
  (Default|Notify (Variables|/Game/LDW/Blueprints/Characters/Player/BP_PlayerControllerGameplay.BP_PlayerControllerGameplay_C|GetPersistentGameplayWBP _asbp_player_controller_gameplay) (Utilities|String|Append "Temple " (Utilities|String|ToString(Integer) (Variables|Default|GetCurrentTempleIndex)) (Utilities|String|SelectString " Boss Fight" (Utilities|String|Append ", Floor " (Utilities|String|ToString(Integer) _floorindexcount)) (>= _floorindexcount (- (Variables|Default|GetNumberOfFloors) 1)))))
  (CallFunction|PlayBGMusic false))

(event EventShutdown
  (bind _currentsavegame (Variables|Default|GetCurrentSaveGame))
  ;[1 1 1] Shutdown
  (Utilities|IsValid _currentsavegame
    (:Is%20Valid
      (Default|AddtoTotalPlayedTime _currentsavegame)
      (SaveGame|SaveGametoSlot _currentsavegame (Variables|Default|GetCurrentSaveSlot)))
    (:Is%20Not%20Valid
      _))
  (Utilities|FlowControl|Delay 2.0)
  (|CallParentFunction))

(event EventLoadSettings
  ;[1 1 1] LoadSettings
  (|CallParentFunction)
  (bind _returnvalue (Settings|GetGameUserSettings))
  (bind _ascustom_game_user_settings (Utilities|Casting|CastToCustomGameUserSettings _returnvalue))
  (Class|GameUserSettings|SetOverallScalabilityLevel _ascustom_game_user_settings (Class|CustomGameUserSettings|GetOverallGraphicSettings _ascustom_game_user_settings))
  (Class|GameUserSettings|ApplySettings _ascustom_game_user_settings false)
  (Class|GameUserSettings|SetVSyncEnabled _ascustom_game_user_settings false)
  (Development|ExecuteConsoleCommand "t.maxfps 240" 0))

(fn CompleteCurrentObjective
  (bind _returnvalue (|CallParentFunction))
  (if _returnvalue
    (bind _asbp_player_controller_gameplay (Utilities|Casting|CastToBP_PlayerControllerGameplay (Game|GetPlayerController 0)))
    (Default|HandlePosCompleteObjective _asbp_player_controller_gameplay)
    (return _returnvalue)
    (else
      (return false))))