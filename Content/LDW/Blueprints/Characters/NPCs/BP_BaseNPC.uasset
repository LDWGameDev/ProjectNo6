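; Base NPC character that acts as a merchant, offering three random, unique floor upgrades picked at BeginPlay.
; An outer thinking sphere shows a world interaction widget to the human player, and an inner interaction sphere switches its state and registers the NPC as interactable with the player controller.
; Pressing E opens the controller's NPC dialog with a random greeting and freshly constructed upgrade objects, switching input to UI only.
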(event OnComponentBeginOverlap(NPCThinkingSphere)
  (params (OverlappedComponent :type Primitive%20Component%20Object%20Reference) (OtherActor :type Actor%20Object%20Reference) (OtherComp :type Primitive%20Component%20Object%20Reference) (OtherBodyIndex :type Integer) (bFromSweep :type Boolean) (SweepResult :type Hit%20Result%20Structure%20%28by%20ref%29))
  (Utilities|Casting|CastToBP_CharacterPlayerHuman OtherActor)
  (bind _npcinteractionwidget (Utilities|GetInteractionWidget)
    (:Success
      (Default|SetEnablingState _npcinteractionwidget true)
      (Default|SetInteractionIndex _npcinteractionwidget))))

(event OnComponentEndOverlap(NPCThinkingSphere)
  (params (OverlappedComponent :type Primitive%20Component%20Object%20Reference) (OtherActor :type Actor%20Object%20Reference) (OtherComp :type Primitive%20Component%20Object%20Reference) (OtherBodyIndex :type Integer))
  (Utilities|Casting|CastToBP_CharacterPlayerHuman OtherActor)
  (bind _npcinteractionwidget (Utilities|GetInteractionWidget)
    (:Success
      (Default|SetEnablingState _npcinteractionwidget false))))

(event OnComponentBeginOverlap(InteractionSphere)
  (params (OverlappedComponent :type Primitive%20Component%20Object%20Reference) (OtherActor :type Actor%20Object%20Reference) (OtherComp :type Primitive%20Component%20Object%20Reference) (OtherBodyIndex :type Integer) (bFromSweep :type Boolean) (SweepResult :type Hit%20Result%20Structure%20%28by%20ref%29))
  (Utilities|Casting|CastToBP_CharacterPlayerHuman OtherActor)
  (bind _npcinteractionwidget (Utilities|GetInteractionWidget)
    (:Success
      (Default|SetInteractionIndex _npcinteractionwidget 1)
      (Class|PlayerControllerGameplay|AddInteractableActor (.AsBP%20Player%20Controller%20Gameplay (Utilities|Casting|CastToBP_PlayerControllerGameplay (Game|GetPlayerController 0))) self))))

(event OnComponentEndOverlap(InteractionSphere)
  (params (OverlappedComponent :type Primitive%20Component%20Object%20Reference) (OtherActor :type Actor%20Object%20Reference) (OtherComp :type Primitive%20Component%20Object%20Reference) (OtherBodyIndex :type Integer))
  (Utilities|Casting|CastToBP_CharacterPlayerHuman OtherActor)
  (bind _npcinteractionwidget (Utilities|GetInteractionWidget)
    (:Success
      (Default|SetInteractionIndex _npcinteractionwidget)
      (Class|PlayerControllerGameplay|RemoveInteractableActor (.AsBP%20Player%20Controller%20Gameplay (Utilities|Casting|CastToBP_PlayerControllerGameplay (Game|GetPlayerController 0))) self))))

(event EventBeginPlay
  (|CallParentFunction)
  (Variables|Default|SetUpgradesInStore (Class|CustomFunctionLibrary|GenerateRandomUniqueIndexesArray 3 (Utilities|Array|LastIndex (Variables|Default|GetFloorUpgradesArray)))))

(fn ConstructionScript)

(fn CreateUpgrades
  (for _array_element (Variables|Default|GetUpgradesInStore)
    (bind _returnvalue (Game|ConstructObjectfromClass (Utilities|Array|Get(acopy) (Variables|Default|GetFloorUpgradesArray) _array_element)))
    (Utilities|Array|Add (LocalVariables|GetTempUpgrades) _returnvalue))
  (return (LocalVariables|GetTempUpgrades)))

(fn TriggerInteractionKey
  (params (PlayerControllerDoTrigger :type Player%20Controller%20Object%20Reference) (Key :type Key%20Structure%20%28by%20ref%29 :default "None"))
  (if (== Key "E")
    (bind _asbp_player_controller_gameplay (Utilities|Casting|CastToBP_PlayerControllerGameplay PlayerControllerDoTrigger)
      (:then
        (Default|SetEnablingState (Variables|/Game/LDW/Blueprints/Characters/Player/BP_PlayerControllerGameplay.BP_PlayerControllerGameplay_C|GetNPCInteractionWBP _asbp_player_controller_gameplay) true)
        (Default|SetChatContent (Variables|/Game/LDW/Blueprints/Characters/Player/BP_PlayerControllerGameplay.BP_PlayerControllerGameplay_C|GetNPCInteractionWBP _asbp_player_controller_gameplay) (.OutItem (Utilities|Array|Random (Variables|Default|GetMerchantGreetingChats))))
        (Input|SetInputModeUIOnly _asbp_player_controller_gameplay (Variables|/Game/LDW/Blueprints/Characters/Player/BP_PlayerControllerGameplay.BP_PlayerControllerGameplay_C|GetNPCInteractionWBP _asbp_player_controller_gameplay) "LockAlways")
        (Default|SetUpgrades (Variables|/Game/LDW/Blueprints/Characters/Player/BP_PlayerControllerGameplay.BP_PlayerControllerGameplay_C|GetNPCInteractionWBP _asbp_player_controller_gameplay) (CallFunction|CreateUpgrades))
        (return true))
      (:CastFailed
        (return false)))))