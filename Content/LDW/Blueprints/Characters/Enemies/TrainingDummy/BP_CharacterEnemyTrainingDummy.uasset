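; Training dummy enemy character that shows damage feedback when hit and dissolves away on death, extending parent damage and death handlers.
; Hits reveal a health bar widget, update it from the HP stat and pop up damage numbers.
; Death ignores pawn and world-dynamic collision, plays a die montage and sound, hides the bar and clears the aura outline.
; A slowed timeline drives the material dissolve, then destroys the actor.
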(event EventBeginPlay)

(event EventHandleDelegateonTookDamage
  (params (DamageDetails :type Damage%20Details%20Object%20Reference))
  (bind _health_bar_widget (Variables|Default|GetHealth%20Bar%20Widget))
  (bind _statcomp (Variables|Default|GetStatComp))
  (bind _returnvalue (Class|StatComponent|GetStat _statcomp "HP"))
  ;[1 1 1] On Took Damage
  (|CallParentFunction DamageDetails)
  (if (not (Variables|Default|GetbIsDeath))
    (if (not (Variables|/Script/Engine.SceneComponent|GetbVisible _health_bar_widget))
      (Rendering|SetVisibility _health_bar_widget true false))
    (bind _aswbp_enemy_health_bar (Utilities|GetHealthBarWidget)
      (:Valid
        (Utilities|IsValid _returnvalue
          (:Is%20Valid
            (Default|UpdateProgressValue _aswbp_enemy_health_bar (Math|Conversions|ToFloat(Integer) (Class|StatBase|GetValue _returnvalue)) (Math|Conversions|ToFloat(Integer) (Variables|/Script/ProjectNo6.StatBase|GetMaxValue _returnvalue)))
            (Default|PopUpDamage (Variables|Default|GetBP%20Damage%20PopUp%20Component) (Variables|/Script/ProjectNo6.DamageDetails|GetDamage DamageDetails))))))))

(event EventOnDied
  ;[1 1 1] On Died
  (|CallParentFunction)
  (Utilities|FlowControl|Sequence
    (:then_0
      (Collision|SetCollisionResponsetoChannel (Variables|Default|GetCapsuleComponent) "ECC_WorldDynamic" "ECR_Ignore")
      (Collision|SetCollisionResponsetoChannel (Variables|Default|GetCapsuleComponent) "ECC_Pawn" "ECR_Ignore")
      (Class|AnimationComponent|PlayCustomMontage (Variables|Default|GetAnimationComp) "die" (Utilities|Name|MakeLiteralName "None") 1.0)
      (Rendering|SetVisibility (Variables|Default|GetHealth%20Bar%20Widget) false false))
    (:then_1
      (Rendering|Material|SetScalarParameterValueonMaterials (Variables|Character|GetMesh) "AuraOutline" 0.0)
      (Components|Timeline|SetPlayRate (Variables|Default|GetDissolveTimeline) 0.25)
      (bind _alpha (Timeline|DissolveTimeline PlayFromStart)
        (:Update
          (Rendering|Material|SetScalarParameterValueonMaterials (Variables|Character|GetMesh) "Dissolve" _alpha))
        (:Finished
          (Actor|DestroyActor))))
    (:then_2
      (Class|CustomFunctionLibrary|CustomSpawnSoundatLocation "enemy_die" (Transformation|GetActorLocation)))))

(fn ConstructionScript)