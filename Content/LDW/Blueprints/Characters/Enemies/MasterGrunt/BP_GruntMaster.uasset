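; Grunt Master boss enemy that plays an activation montage, starts periodic minion spawning through its boss spawner, and shows a boss health bar.
; Damage updates health, the bar and a hit outline.
; Its range attack sphere-traces forward for pawns and triggers an overlap combat move with FX at the hit.
; Death stops AI, clears minions and runs timed dissolve, slow motion, defeat notice and dialogue, and sets the level-completed notification.
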(event Custom|ActivateGruntMaster
  (bind _enemybossspawner (Variables|Default|GetEnemyBossSpawner))
  ;[1 1 1] Activate Master Grunt
  (Class|AnimationComponent|PlayCustomMontage (Variables|Default|GetAnimationComp) "actions" (Utilities|Name|MakeLiteralName "activate") 1.0)
  (Utilities|IsValid _enemybossspawner
    (:Is%20Valid
      (Default|StartSpawningPeriodically _enemybossspawner))))

(event Custom|EndActivation
  ;[1 1 1] End Activation
  (CallFunction|TryActivateEnemy)
  (CallFunction|ShowBossInfo))

(event Custom|SpawnEnemies
  (bind _enemybossspawner (Variables|Default|GetEnemyBossSpawner))
  (Utilities|IsValid _enemybossspawner
    (:Is%20Valid
      (Default|SpawnEnemywithAmountCheck _enemybossspawner))))

(event Custom|RangeAttack
  (bind _returnvalue (Math|Transform|MakeTransform "350.000000, 0,-280.000000" "0, 0, 0" "2.000000,1.500000,1.500000"))
  (bind _returnvalue_2 (Transformation|GetActorLocation))
  (bind _returnvalue_3 (Transformation|GetActorForwardVector))
  (bind _combatcomp (Variables|Default|GetCombatComp))
  ;[1 1 1] Range Attack
  (Class|FXComponent|SpawnFXatLocation (Variables|Default|GetFXComp) "range_attack" (.location _returnvalue) (.rotation _returnvalue) (.scale _returnvalue) true true "None" true)
  (Utilities|FlowControl|Delay 0.2)
  (bind (_outhit _returnvalue_4) (Collision|SphereTraceForObjects (+ (* _returnvalue_3 (Math|Float|MakeLiteralFloat 5e+01)) _returnvalue_2 "0,0,-150.000000") (+ (* _returnvalue_3 (Math|Float|MakeLiteralFloat 1.5e+03)) _returnvalue_2 "0,0,-150.000000") 1.2e+02 (Utilities|Array|MakeArray "ObjectTypeQuery3") false (Utilities|Array|MakeArray self) "None" true "(R=1.000000,G=0.000000,B=0.000000,A=1.000000)" "(R=0.000000,G=1.000000,B=0.000000,A=1.000000)" 1.0))
  (if _returnvalue_4
    (bind _ascombat_move_sphere_overlap (Utilities|Casting|CastToCombatMoveSphereOverlap (Class|CombatComponent|FindCombatMove _combatcomp "range_attack")))
    (Class|CombatMoveSphereOverlap|SphereOverlapSetWorldLocation _ascombat_move_sphere_overlap (.Location (Collision|BreakHitResult _outhit)))
    (Class|CombatComponent|TriggerCombatMove _combatcomp (Variables|/Script/ProjectNo6.CombatMove|GetMoveID _ascombat_move_sphere_overlap))
    (Class|FXComponent|SpawnFXatLocation (Variables|Default|GetFXComp) "range_attack_hit" (+ (* (Transformation|GetActorForwardVector) (Math|Float|MakeLiteralFloat 6e+01)) (Math|Vector|MakeVector (.X (Math|Vector|BreakVector (.Location (Collision|BreakHitResult _outhit)))) (.Y (Math|Vector|BreakVector (.Location (Collision|BreakHitResult _outhit)))) (.z (- (Transformation|GetActorLocation) "0,0,280.000000")))) (Math|Rotator|MakeRotator 0.0 0.0 0.0) "1.250000,1.250000,1.250000" false true "None" true)))

(event EventBeginPlay)

(event EventOnDied
  (bind _enemybossspawner (Variables|Default|GetEnemyBossSpawner))
  ;[1 1 1] On Died
  (if (not (Variables|Default|GetbIsDeath))
    (Utilities|FlowControl|Sequence
      (:then_0
        (Class|AnimationComponent|PlayCustomMontage (Variables|Default|GetAnimationComp) "actions_no_blend_out" (Utilities|Name|MakeLiteralName "die") 1.0)
        (CallFunction|StopBrainLogic)
        (CallFunction|UpdateDeathCollision)
        (CallFunction|TryRemoveCurrentHitboxIndicatorFX)
        (bind _asbp_game_instance_custom (Utilities|Casting|CastToBP_GameInstanceCustom (Game|GetGameInstance)))
        (Variables|/Game/LDW/Blueprints/Game/BP_GameInstanceCustom.BP_GameInstanceCustom_C|SetStartLevelNotification _asbp_game_instance_custom "Completed Cobra Tomb")
        (Utilities|IsValid _enemybossspawner
          (:Is%20Valid
            (Default|DestroyAllSpawnedEnemies _enemybossspawner))))
      (:then_1
        (Utilities|FlowControl|Delay 3.0)
        (CallFunction|PlayDissolveEffect))
      (:then_2
        (Class|CharacterEnemyBase|OndiedCode)
        (CallFunction|HideBossInfo)
        (bind _asbp_game_instance_custom_2 (Utilities|Casting|CastToBP_GameInstanceCustom (Game|GetGameInstance)))
        (Class|GameInstanceCustom|SetTimeDilationforDuration _asbp_game_instance_custom_2 0.1 1.0)
        (Utilities|FlowControl|Delay 0.5)
        (bind _asbp_player_controller_gameplay (Utilities|Casting|CastToBP_PlayerControllerGameplay (Game|GetPlayerController 0)))
        (Default|Notify (Variables|/Game/LDW/Blueprints/Characters/Player/BP_PlayerControllerGameplay.BP_PlayerControllerGameplay_C|GetPersistentGameplayWBP _asbp_player_controller_gameplay) "Defeated Grunt Master"))
      (:then_3
        (Utilities|FlowControl|Delay 5.5)
        (bind _asbp_game_instance_custom_3 (Utilities|Casting|CastToBP_GameInstanceCustom (Game|GetGameInstance)))
        (Default|StartNewDialogue _asbp_game_instance_custom_3)))))

(event EventHandleDelegateonTookDamage
  (params (DamageDetails :type Damage%20Details%20Object%20Reference))
  (if (not (Variables|Default|GetbIsDeath))
    (Class|CharacterEnemyBase|ReduceHealthwhenGetHit DamageDetails)
    (Class|CharacterEnemyBase|PlayGetHitOutlineEffect 3.0)
    (CallFunction|UpdateBossHealthBar)))

(fn ConstructionScript
  (|CallParentFunction))

(fn ShowBossInfo
  (bind _asbp_player_controller_gameplay (Utilities|Casting|CastToBP_PlayerControllerGameplay (Game|GetPlayerController 0)))
  (Default|ShowBossInfo (Variables|/Game/LDW/Blueprints/Characters/Player/BP_PlayerControllerGameplay.BP_PlayerControllerGameplay_C|GetPersistentGameplayWBP _asbp_player_controller_gameplay) "Grunt Master")
  (CallFunction|UpdateBossHealthBar))

(fn UpdateBossHealthBar
  (bind _statcomp (Variables|Default|GetStatComp))
  (bind _returnvalue (Class|StatComponent|GetStat _statcomp "HP"))
  (Utilities|IsValid _returnvalue
    (:Is%20Valid
      (bind _asbp_player_controller_gameplay (Utilities|Casting|CastToBP_PlayerControllerGameplay (Game|GetPlayerController 0)))
      (Default|UpdateBossHealth (Variables|/Game/LDW/Blueprints/Characters/Player/BP_PlayerControllerGameplay.BP_PlayerControllerGameplay_C|GetPersistentGameplayWBP _asbp_player_controller_gameplay) (Class|StatBase|GetValue _returnvalue) (Variables|/Script/ProjectNo6.StatBase|GetMaxValue _returnvalue)))))

(fn HideBossInfo
  (bind _asbp_player_controller_gameplay (Utilities|Casting|CastToBP_PlayerControllerGameplay (Game|GetPlayerController 0)))
  (Default|HideBossInfo (Variables|/Game/LDW/Blueprints/Characters/Player/BP_PlayerControllerGameplay.BP_PlayerControllerGameplay_C|GetPersistentGameplayWBP _asbp_player_controller_gameplay)))