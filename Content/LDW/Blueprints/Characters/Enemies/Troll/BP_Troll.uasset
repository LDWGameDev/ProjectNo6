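; BP_Troll is the troll enemy Blueprint, extending a parent enemy class with its activation and death behavior.
; When parent activation succeeds, it plays an activate montage through AnimationComp and rotates to face the player.
; On death, it runs the parent logic, plays a die montage from a no-blend montage and removes any current hitbox indicator effect.
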(event EventOnDied
  (|CallParentFunction)
  (Class|AnimationComponent|PlayCustomMontage (Variables|Default|GetAnimationComp) "actions_no_blend" (Utilities|Name|MakeLiteralName "die") 1.0)
  (CallFunction|TryRemoveCurrentHitboxIndicatorFX))

(fn ConstructionScript
  (|CallParentFunction))

(fn TryActivateEnemy
  (bind _bsuccess (|CallParentFunction))
  (if _bsuccess
    (Class|AnimationComponent|PlayCustomMontage (Variables|Default|GetAnimationComp) "actions" (Utilities|Name|MakeLiteralName "activate") 1.0)
    (CallFunction|RotatetoFacePlayer 0.2)
    (return true)
    (else
      (return false))))