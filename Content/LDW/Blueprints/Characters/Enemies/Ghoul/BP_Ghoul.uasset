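; Ghoul enemy character Blueprint that adds its own hit, death and activation reactions on top of the parent enemy logic.
; When hit, it turns toward the attacker, steps back (less for light hits), plays a get-hit montage and finishes its active movement task.
; On death it plays a die montage; on activation it roars and briefly suppresses hit reactions.
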(event EventBeginPlay
  (|CallParentFunction))

(event EventHandleDelegateonTookDamage
  (params (DamageDetails :type Damage%20Details%20Object%20Reference))
  ;[1 1 1] On Took Damage
  (|CallParentFunction DamageDetails)
  (if (not (Variables|Default|GetbIsDeath))
    (Utilities|FlowControl|Sequence
      (:then_0
        (if (Variables|Default|GetbCanVisualizeGetHitAction)
          (Class|CharacterEnemyBase|RotatetoFaceInstigatorwhenGetHit DamageDetails)
          (CallFunction|GetHitStepBack DamageDetails)
          (Class|AnimationComponent|PlayCustomMontage (Variables|Default|GetAnimationComp) "actions" (Utilities|Name|MakeLiteralName "get_hit") 1.0)
          (CallFunction|FinishCurrentTaskifIsMovement true "/Game/LDW/Blueprints/Characters/Enemies/BTTask_MoveToPlayer.BTTask_MoveToPlayer_C")
          (CallFunction|FinishCurrentTaskifIsMovement true "/Game/LDW/Blueprints/Characters/Enemies/BTTask_MoveRandomInRange.BTTask_MoveRandomInRange_C"))))))

(event EventOnDied
  ;[1 1 1] On Died
  (|CallParentFunction)
  (Utilities|FlowControl|Sequence
    (:then_0
      (Class|AnimationComponent|PlayCustomMontage (Variables|Default|GetAnimationComp) "die" (Utilities|Name|MakeLiteralName "die") 1.0))))

(fn ConstructionScript)

(fn GetHitStepBack
  (params (Damage%20Details :type Damage%20Details%20Object%20Reference))
  (bind _instigatorcombatmove (Variables|/Script/ProjectNo6.DamageDetails|GetInstigatorCombatMove Damage%20Details))
  (LocalVariables|SetStepBackDistance 6e+01)
  (Utilities|IsValid _instigatorcombatmove
    (:Is%20Valid
      (if (Utilities|Enum|Equal(Enum) (Variables|/Script/ProjectNo6.CombatMove|GetHitType _instigatorcombatmove) "LightHit")
        (LocalVariables|SetStepBackDistance 4e+01))
      (Class|CharacterEnemyBase|StepBackwhenGetHit Damage%20Details (LocalVariables|GetStepBackDistance)))))

(fn TryActivateEnemy
  (bind _bsuccess (|CallParentFunction))
  (if _bsuccess
    (Class|AnimationComponent|PlayCustomMontage (Variables|Default|GetAnimationComp) "actions" (Utilities|Name|MakeLiteralName "roar") 1.0)
    (CallFunction|DisableVisualizingGetHitActionforDuration 1.0)
    (return true)
    (else
      (return false))))