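; Lich enemy character that extends a parent enemy class with a ranged beam spell and its own activation, hit and death reactions.
; StartRangeAttack drives a forward Niagara beam from a timeline while a looping timer sphere-traces along it, moving the range_spell combat move to each hit and triggering it with blood FX.
; Taking damage can turn the Lich, step it back by hit type, play a montage and finish its movement tasks.
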(event Custom|StartRangeAttack
  (bind _returnvalue (Transformation|GetActorLocation))
  (bind _rangeattackniasyscomp (Variables|Default|GetRangeAttackNiaSysComp))
  (bind _combatcomp (Variables|Default|GetCombatComp))
  (bind _rangeattackniasyscomp_2 (Variables|Default|GetRangeAttackNiaSysComp))
  (Niagara|SetNiagaraVariable(Vector3) _rangeattackniasyscomp_2 "End" (+ (Transformation|GetWorldLocation _rangeattackniasyscomp_2) (* (Transformation|GetActorForwardVector) (Math|Float|MakeLiteralFloat 1.2e+03))))
  (Niagara|SetNiagaraVariable(Float) _rangeattackniasyscomp_2 "Size" 0.2)
  (Utilities|FlowControl|Delay 0.0)
  (Utilities|FlowControl|Delay 0.0)
  (Rendering|SetVisibility (Variables|Default|GetRangeAttackNiaSysComp) true false)
  (Components|Timeline|SetPlayRate (Variables|Default|GetRangeAttackTimeline) 0.5)
  (Utilities|FlowControl|Sequence
    (:then_0
      (bind _distancemultiplier (Timeline|RangeAttackTimeline PlayFromStart)
        (:Update
          (Niagara|SetNiagaraVariable(Vector3) _rangeattackniasyscomp "End" (+ (Transformation|GetActorLocation) (* (Transformation|GetActorForwardVector) (Math|Float|MakeLiteralFloat 1.2e+03)) "0,0,-20.000000"))
          (Niagara|SetNiagaraVariable(Float) _rangeattackniasyscomp "Size" _distancemultiplier))
        (:Finished
          (Rendering|SetVisibility (Variables|Default|GetRangeAttackNiaSysComp) false false)
          (Utilities|Time|ClearandInvalidateTimerbyHandle (Variables|Default|GetLongSpellTraceTargetTimerHandle)))))
    (:then_1
      (bind _returnvalue_2 (Utilities|Time|SetTimerbyEvent (delegate Custom|RangeAttackTraceTarget) 0.3 true))
      (Variables|Default|SetLongSpellTraceTargetTimerHandle _returnvalue_2)
      (bind (_outhit _returnvalue_3) (Collision|SphereTraceForObjects _returnvalue (+ _returnvalue (* (Transformation|GetActorForwardVector) (Math|Float|MakeLiteralFloat 1.2e+03))) 5e+01 (Utilities|Array|MakeArray "ObjectTypeQuery3" "ObjectTypeQuery1" "ObjectTypeQuery2") false (Utilities|Array|MakeArray self) "None" true "(R=1.000000,G=0.000000,B=0.000000,A=1.000000)" "(R=0.000000,G=1.000000,B=0.000000,A=1.000000)" 2.0))
      (if _returnvalue_3
        (bind _ascombat_move_sphere_overlap (Utilities|Casting|CastToCombatMoveSphereOverlap (Class|CombatComponent|FindCombatMove _combatcomp "range_spell")))
        (Class|CombatMoveSphereOverlap|SphereOverlapSetWorldLocation _ascombat_move_sphere_overlap (.Location (Collision|BreakHitResult _outhit)))
        (Class|CombatComponent|TriggerCombatMove _combatcomp "range_spell")
        (Niagara|SpawnSystematLocation "/Game/ImproveFights_Vfx/Particles/P_GeneralHIt_Blood.P_GeneralHit_Blood" (.Location (Collision|BreakHitResult _outhit)))))))

(event Custom|EndRangeAttack)

(event Custom|RangeAttackTraceTarget
  (bind _returnvalue (Transformation|GetActorLocation))
  (bind _combatcomp (Variables|Default|GetCombatComp))
  (bind (_outhit _returnvalue_2) (Collision|SphereTraceForObjects _returnvalue (+ _returnvalue (* (Transformation|GetActorForwardVector) (Math|Float|MakeLiteralFloat 1.2e+03))) 5e+01 (Utilities|Array|MakeArray "ObjectTypeQuery3" "ObjectTypeQuery1" "ObjectTypeQuery2") false (Utilities|Array|MakeArray self) "None" true "(R=1.000000,G=0.000000,B=0.000000,A=1.000000)" "(R=0.000000,G=1.000000,B=0.000000,A=1.000000)" 2.0))
  (if _returnvalue_2
    (bind _ascombat_move_sphere_overlap (Utilities|Casting|CastToCombatMoveSphereOverlap (Class|CombatComponent|FindCombatMove _combatcomp "range_spell")))
    (Class|CombatMoveSphereOverlap|SphereOverlapSetWorldLocation _ascombat_move_sphere_overlap (.Location (Collision|BreakHitResult _outhit)))
    (Class|CombatComponent|TriggerCombatMove _combatcomp "range_spell")
    (Niagara|SpawnSystematLocation "/Game/ImproveFights_Vfx/Particles/P_GeneralHIt_Blood.P_GeneralHit_Blood" (.Location (Collision|BreakHitResult _outhit)))))

(event EventBeginPlay
  (|CallParentFunction))

(event EventHandleDelegateonTookDamage
  (params (DamageDetails :type Damage%20Details%20Object%20Reference))
  (|CallParentFunction DamageDetails)
  (if (not (Variables|Default|GetbIsDeath))
    (Utilities|FlowControl|Sequence
      (:then_0
        (if (Variables|Default|GetbCanVisualizeGetHitAction)
          (Class|CharacterEnemyBase|RotatetoFaceInstigatorwhenGetHit DamageDetails)
          (CallFunction|GetHitStepBack DamageDetails)
          (Class|AnimationComponent|PlayCustomMontage (Variables|Default|GetAnimationComp) "actions" (Utilities|Name|MakeLiteralName "get_hit") 1.0)
          (CallFunction|FinishCurrentTaskifIsMovement true "/Game/LDW/Blueprints/Characters/Enemies/BTTask_MoveToPlayer.BTTask_MoveToPlayer_C")
          (CallFunction|FinishCurrentTaskifIsMovement true "/Game/LDW/Blueprints/Characters/Enemies/BTTask_MoveRandomInRange.BTTask_MoveRandomInRange_C")
          (CallFunction|TryRemoveCurrentHitboxIndicatorFX))))))

(event EventOnDied
  (|CallParentFunction)
  (Class|AnimationComponent|PlayCustomMontage (Variables|Default|GetAnimationComp) "actions_no_blend_out" (Utilities|Name|MakeLiteralName "die") 1.0)
  (Audio|PlaySound2D "/Game/LDW/Assets/Sounds/S_LichDie.S_LichDie" 1.0 1.0 0.0 0 0)
  (CallFunction|TryRemoveCurrentHitboxIndicatorFX))

(fn ConstructionScript
  (|CallParentFunction))

(fn TryActivateEnemy
  (bind _bsuccess (|CallParentFunction))
  (if _bsuccess
    (Class|AnimationComponent|PlayCustomMontage (Variables|Default|GetAnimationComp) "actions" (Utilities|Name|MakeLiteralName "activate") 1.0)
    (CallFunction|DisableVisualizingGetHitActionforDuration 2.0)
    (Audio|PlaySound2D "/Game/LDW/Assets/Sounds/S_LichActivate.S_LichActivate" 1.0 1.0 0.0 0 0)
    (return true)
    (else
      (return false))))

(fn GetHitStepBack
  (params (Damage%20Details :type Damage%20Details%20Object%20Reference))
  (bind _instigatorcombatmove (Variables|/Script/ProjectNo6.DamageDetails|GetInstigatorCombatMove Damage%20Details))
  (Utilities|IsValid Damage%20Details
    (:Is%20Valid
      (Utilities|IsValid _instigatorcombatmove
        (:Is%20Valid
          (LocalVariables|SetStepBackDistance 6e+01)
          (if (Utilities|Enum|Equal(Enum) (Variables|/Script/ProjectNo6.CombatMove|GetHitType _instigatorcombatmove) "LightHit")
            (LocalVariables|SetStepBackDistance 4e+01))
          (Class|CharacterEnemyBase|StepBackwhenGetHit Damage%20Details (LocalVariables|GetStepBackDistance)))))))