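; BP_PlayerControllerMainMenu is the player controller for the main menu, which builds the menu UI when play begins.
; It creates WBP_MainMenu, adds it to the viewport, switches to UI-only input focused on that widget and shows the mouse cursor.
; It also creates a WBP_Transition widget layered above the menu and keeps references to both widgets.
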(event EventBeginPlay
  (|CallParentFunction)
  (Utilities|FlowControl|Sequence
    (:then_0
      (bind _returnvalue (UserInterface|CreateWidget "/Game/LDW/Blueprints/Widgets/MainMenu/WBP_MainMenu.WBP_MainMenu_C" self))
      (bind _output_get (Variables|Default|SetMainMenuWidget _returnvalue))
      (UserInterface|Viewport|AddtoViewport _output_get 15)
      (Input|SetInputModeUIOnly self _output_get "DoNotLock")
      (Variables|Default|SetbShowMouseCursor true))
    (:then_1
      (bind _returnvalue_2 (UserInterface|CreateWidget "/Game/LDW/Blueprints/Widgets/WBP_Transition.WBP_Transition_C" self))
      (bind _output_get_2 (Variables|Default|SetTransitionWidget _returnvalue_2))
      (UserInterface|Viewport|AddtoViewport _output_get_2 20))))

(fn ConstructionScript)