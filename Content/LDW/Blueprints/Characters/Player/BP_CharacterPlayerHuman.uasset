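; Human player character Blueprint that layers visual, audio and UI feedback onto inherited combat events.
; Equipment changes drive the torch light, fading in by timeline then flickering via a looping curve timer, plus weapon-slot and under-foot direction widgets.
; Hits, perfect dashes and death trigger screen effects, sounds, slow motion or the death screen.
; It also handles stamina widgets, camera views, enemy snap assist and debug spline-trail testing.
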(event Custom|HandleOnEquipmentIndexChangedDelegate
  (params (OldType :type EHoldingObjectType%20Enum :default "None") (NewType :type EHoldingObjectType%20Enum :default "None"))
  ;[1 1 1] Begin Play
  (CallFunction|OnEquipmentIndexChanged OldType NewType))

(event Custom|TorchStartBurning
  ;[1 1 1] Torch Start Burning
  (bind _intensity_alpha (Timeline|Timeline_DrawTorch PlayFromStart)
    (:Update
      (if (Utilities|Enum|Equal(Enum) (Variables|/Script/ProjectNo6.EquipmentComponent|GetCurrentHoldingType (Variables|Default|GetEquipComp)) "Torch")
        (Rendering|Components|Light|SetIntensity (Variables|Default|GetTorchPointLightComp) (Math|Float|Lerp 0.0 (Variables|TorchLight|GetTorchPointLightIntensity) _intensity_alpha))
        (else
          (Audio|Components|Audio|Stop (Variables|Default|GetTimeline_DrawTorch)))))
    (:Finished
      ;;[1 1 1] Torch fire flickering
      (if (Utilities|Enum|Equal(Enum) (Variables|/Script/ProjectNo6.EquipmentComponent|GetCurrentHoldingType (Variables|Default|GetEquipComp)) "Torch")
        (if (Utilities|Time|IsTimerActivebyHandle (Variables|TorchLight|GetTorchFlickeringTimerHandle))
          (Utilities|Time|ClearandInvalidateTimerbyHandle (Variables|TorchLight|GetTorchFlickeringTimerHandle)))
        (bind _returnvalue (Utilities|Time|SetTimerbyEvent (delegate Custom|HandleTimer_TorchFlickering) (Math|Float|MakeLiteralFloat 0.15) true))
        (Variables|TorchLight|SetTorchFlickeringTimerHandle _returnvalue)
        (Variables|TorchLight|SetTorchAlphaCounter 0.0)))))

(event Custom|HandleTimer_TorchFlickering
  (bind _torchflickeringtimerhandle (Variables|TorchLight|GetTorchFlickeringTimerHandle))
  ;[1 1 1] Torch Start Burning
  (if (Utilities|Enum|Equal(Enum) (Variables|/Script/ProjectNo6.EquipmentComponent|GetCurrentHoldingType (Variables|Default|GetEquipComp)) "Torch")
    (bind _output_get (Variables|TorchLight|SetTorchAlphaCounter (Math|Float|SelectFloat 0.0 (+ (Variables|TorchLight|GetTorchAlphaCounter) (Math|Float|MakeLiteralFloat 0.15)) (> (+ (Variables|TorchLight|GetTorchAlphaCounter) (Math|Float|MakeLiteralFloat 0.15)) 4.0))))
    (Rendering|Components|Light|SetIntensity (Variables|Default|GetTorchPointLightComp) (Math|Float|MapRangeUnclamped (Math|Curves|GetFloatValue (Variables|TorchLight|GetTorchFlickeringCurve) _output_get) 0.0 1.0 0.0 (Variables|TorchLight|GetTorchPointLightIntensity)))
    (elif (Utilities|Time|IsTimerActivebyHandle _torchflickeringtimerhandle)
      (Utilities|Time|ClearandInvalidateTimerbyHandle _torchflickeringtimerhandle))))

(event Custom|SpawnSFX
  (params (Id :type String) (Location :type Vector))
  ;[1 1 1] Spawn SFX
  (Class|CustomFunctionLibrary|CustomSpawnSoundatLocation Id Location))

(event Custom|TestSplineTrail
  (params (Duration :type Float%20%28double-precision%29))
  (bind _returnvalue (Class|FXComponent|SpawnFXatLocation (Variables|Default|GetFXComp) "sword_trail" (Transformation|GetActorLocation) (Transformation|GetActorRotation) "1.000000,1.000000,1.000000" true false "None" true))
  (Utilities|FlowControl|Sequence
    (:then_0
      (Variables|Default|SetTesting_LastFXLocation (Spline|GetLocationatTime (Variables|Default|GetSpline) 0.0 "World" false))
      (Components|Timeline|SetPlayRate (Variables|Default|GetTimeline_0) (Math|Float|SafeDivide 1.0 Duration))
      (bind _alpha (Timeline|Timeline_0 PlayFromStart)
        (:Update
          (Utilities|IsValid _returnvalue
            (:Is%20Valid
              (Transformation|SetWorldLocation _returnvalue (Spline|GetLocationatTime (Variables|Default|GetSpline) _alpha "World" false) false false)
              (Utilities|IsValid (Variables|/Script/ProjectNo6.EquipmentComponent|GetTorchHoldingActor (Class|CharacterPlayerBase|GetEquipmentComp))
                (:Is%20Valid
                  (Transformation|SetWorldRotation _returnvalue (Math|Rotator|MakeRotfromXZ (Math|Vector|Normalize (- (Spline|GetLocationatTime (Variables|Default|GetSpline) _alpha "World" false) (Variables|Default|GetTesting_LastFXLocation))) (Math|Vector|Normalize (- (Spline|GetLocationatTime (Variables|Default|GetSpline) _alpha "World" false) (Transformation|GetActorLocation)))) false false)
                  (Variables|Default|SetTesting_LastFXLocation (Spline|GetLocationatTime (Variables|Default|GetSpline) _alpha "World" false)))))))
        (:Finished
          (Utilities|FlowControl|Delay 1.0)
          (Components|DestroyComponent _returnvalue)
          (Utilities|Time|SetGlobalTimeDilation 1.0))))
    (:then_1
      (Utilities|Time|SetGlobalTimeDilation 1.0))))

(event Custom|CustomEvent_0)

(event Custom|EnableSparkling
  (params (bDoEnable :type Boolean) (SocketName :type Name) (RelativeLocation :type Vector))
  (bind _returnvalue (Class|CharacterPlayerBase|GetFXComponent))
  (bind _sparklewidgetcomp (Variables|/Script/ProjectNo6.FXComponent|GetSparkleWidgetComp _returnvalue))
  ;[1 1 1] Enable Sparkling
  (if (and (Utilities|IsValid _returnvalue) (Utilities|IsValid _sparklewidgetcomp))
    (Utilities|FlowControl|Sequence
      (:then_0
        (bind _aswbp_single_sparkle (Utilities|Casting|CastToWBP_SingleSparkle (UserInterface|GetWidget _sparklewidgetcomp)))
        (if bDoEnable
          (Default|EnableSparkling _aswbp_single_sparkle)
          (else
            (Default|DisableSparkling _aswbp_single_sparkle))))
      (:then_1
        (Transformation|AttachComponentToComponent _sparklewidgetcomp (Variables|Character|GetMesh) SocketName "KeepWorld" "KeepWorld" "KeepRelative" true)
        (Transformation|SetRelativeLocation _sparklewidgetcomp RelativeLocation false false))
      (:then_2
        (Rendering|SetVisibility _sparklewidgetcomp bDoEnable false)))))

(event Custom|NotifyWithOverHeadNotification
  (params (Content :type Text) (TypeIndex :type Integer))
  ;[1 1 1] Notify With Over Head Notification
  (bind _aswbp_over_head_notification (Utilities|Casting|CastToWBP_OverHeadNotification (UserInterface|GetWidget (Variables|Default|GetOverHeadNotification))))
  (Default|ShowNotification _aswbp_over_head_notification Content TypeIndex))

(event Custom|ClearFloorUpgradesArray
  ;[1 1 1] Clear Floor Upgrades
  (for _array_element (Variables|Default|GetFloorUpgradesArray)
    (Default|StopEffect _array_element (.AsBP%20Player%20Controller%20Gameplay (Utilities|Casting|CastToBP_PlayerControllerGameplay (Pawn|GetController)))))
  (Utilities|Array|Clear (Variables|Default|GetFloorUpgradesArray)))

(event Custom|SetCameraView
  (params (ViewIndex :type Integer))
  (bind _returnvalue (Pawn|GetController))
  (bind _asplayer_controller (Utilities|Casting|CastToPlayerController _returnvalue))
  ;[1 1 1] Set Camera View
  (Utilities|Casting|CastToPlayerController (Pawn|GetController))
  (switch int ViewIndex
    (:0
      (Game|Player|SetViewTargetwithBlend _asplayer_controller self 0.75 "VTBlend_Linear" 0.0 true))
    (:1
      (Game|Player|SetViewTargetwithBlend _asplayer_controller (Variables|/Script/Engine.ChildActorComponent|GetChildActor (Variables|Default|GetZoomCamChild)) 0.75 "VTBlend_Linear" 0.0 true))))

(event Input|EnhancedActionEvents|EnhancedInputActionIA_Reset
  (params (ActionValue :type Boolean) (ElapsedSeconds :type Float%20%28double-precision%29) (TriggeredSeconds :type Float%20%28double-precision%29) (InputAction :type Input%20Action%20Object%20Reference :default "/Game/LDW/Blueprints/EnhancedInput/IA_Reset.IA_Reset")))

(event EventTick
  (params (DeltaSeconds :type Float%20%28single-precision%29))
  ;[1 1 1] Event Tick
  (|CallParentFunction DeltaSeconds))

(event EventBeginPlay
  ;[1 1 1] Begin Play
  (|CallParentFunction)
  (Utilities|FlowControl|Sequence
    (:then_0
      (EventDispatchers|AssignOnEquipmentIndexChangedDelegate (Variables|Default|GetEquipComp) (delegate Custom|HandleOnEquipmentIndexChangedDelegate)))
    (:then_1
      (bind _aswbp_persistent_stamina (Utilities|Casting|CastToWBP_PersistentStamina (UserInterface|GetWidget (Variables|Default|GetPersistentStaminaWidgetComp))))
      (Variables|Default|SetPersistentStaminaWidget _aswbp_persistent_stamina)
      (bind _aswbp_under_foot_direction (Utilities|Casting|CastToWBP_UnderFootDirection (UserInterface|GetWidget (Variables|Default|GetUnderFootDirectionWidgetComp))))
      (Variables|Default|SetUnderFootDirectionWidget _aswbp_under_foot_direction))
    (:then_2
      (for _array_element (Actor|GetComponentsByClass "/Script/UMG.WidgetComponent")
        (Collision|SetCollisionEnabled _array_element "NoCollision")))
    (:then_3
      (Utilities|FlowControl|Delay 0.75)
      (Class|EquipmentComponent|SetCurrentHoldingType (Variables|Default|GetEquipComp) "GunSword" false))))

(event EventUnderFootDirectionEffect
  (params (Duration :type Float%20%28single-precision%29))
  ;[1 1 1] Under Foot Direction Effect
  (if (> Duration 0.0)
    (bind _underfootdirectionwidget (Utilities|GetUnderFootDirectionWidget)
      (:Valid
        (Default|TriggerEnable _underfootdirectionwidget Duration)))))

(event EventUpdateStamineGemsAmount
  (params (Amount :type Integer))
  ;[1 1 1] Update Stamina Gems Amount
  (|CallParentFunction Amount)
  (bind _aswbp_persistent_stamina (Utilities|Casting|CastToWBP_PersistentStamina (UserInterface|GetWidget (Variables|Default|GetPersistentStaminaWidgetComp))))
  (Default|UpdateStaminaGemsNumber _aswbp_persistent_stamina Amount))

(event EventUpdateStaminaGemState
  (params (bIncreased :type Boolean))
  (bind _statcomp (Variables|Default|GetStatComp))
  (bind _powerstat (Variables|/Script/ProjectNo6.StatComponent|GetPowerStat _statcomp))
  ;[1 1 1] Update Stamina Gem State
  (|CallParentFunction bIncreased)
  (Utilities|IsValid _statcomp
    (:Is%20Valid
      (if (and (Utilities|IsValid _powerstat) (Utilities|IsValid (Variables|Default|GetPersistentStaminaWidget)))
        (Default|UpdateStaminaGemState (Variables|Default|GetPersistentStaminaWidget) bIncreased (Class|StatBase|GetValue _powerstat))))))

(event EventOnGetHit
  (params (DamageDetails :type Damage%20Details%20Object%20Reference))
  ;[1 1 1] On Get Hit
  (|CallParentFunction DamageDetails)
  (if (not (Variables|Default|GetbIsDeath))
    (bind _as_bp_gameplay_controller (Utilities|GetGameplayController)
      (:Valid
        (Default|ShowBloodScreen _as_bp_gameplay_controller)
        (CallFunction|PlayCameraShake "/Game/LDW/Blueprints/Data/CameraShake/CS_ShortLightShake2.CS_ShortLightShake2_C")
        (Class|CustomFunctionLibrary|CustomSpawnSoundatLocation "player_get_hit" (Transformation|GetActorLocation))
        (Audio|PlaySound2D "/Game/Art/Imports/Sounds/SFXs/Wukong_SFX/WAV/Stick_Impact/punch_grit_wet_impact_05.punch_grit_wet_impact_05" (Math|Random|RandomFloatinRange 0.8 1.2) (Math|Random|RandomFloatinRange 0.8 1.2) 0.0 0 0)))))

(event EventOnEvadeAttackwithDashing
  (params (DamageDetails :type Damage%20Details%20Object%20Reference))
  ;[1 1 1] On Evade Attack With Dashing
  (|CallParentFunction DamageDetails)
  (bind _asbp_game_instance_custom (Utilities|Casting|CastToBP_GameInstanceCustom (Game|GetGameInstance)))
  (Class|GameInstanceCustom|SetTimeDilationforDuration _asbp_game_instance_custom 0.1 0.25)
  (Utilities|FlowControl|Delay 0.25)
  (Audio|SpawnSound2D "/Game/LDW/Assets/Sounds/S_DashEvadeGettingHit.S_DashEvadeGettingHit" 1.0 1.0 0.0 0)
  (CallFunction|NotifywithOverHeadNotification "Perfect Dash"))

(event EventOnDied
  (bind _returnvalue (Game|GetPlayerController 0))
  ;[1 1 1] On Died
  (|CallParentFunction)
  (Utilities|FlowControl|Sequence
    (:then_0
      (bind _returnvalue_2 (UserInterface|CreateWidget "/Game/LDW/Blueprints/Widgets/WBP_PlayerDeathScreen.WBP_PlayerDeathScreen_C" _returnvalue))
      (UserInterface|Viewport|AddtoViewport _returnvalue_2 50)
      (Input|SetInputModeUIOnly _returnvalue _returnvalue_2 "DoNotLock")
      (Variables|/Script/Engine.PlayerController|SetbShowMouseCursor _returnvalue true)
      (Audio|PlaySound2D "/Game/Art/Imports/Sounds/SFXs/Wukong_SFX/WAV/Stick_Impact/punch_grit_wet_impact_05.punch_grit_wet_impact_05" 1.0 1.0 0.0 0 0)
      (Class|CharacterPlayerBase|CustomPlaySound "player_exhausted_effort_groan" (Transformation|GetActorLocation)))
    (:then_1
      (Class|AnimationComponent|PlayCustomMontage (Variables|Default|GetAnimationComp) "die" (Utilities|Name|MakeLiteralName "die") 1.0)
      (bind _asbp_player_controller_gameplay (Utilities|Casting|CastToBP_PlayerControllerGameplay (Game|GetPlayerController 0)))
      (Default|RemoveUpgrades (Variables|/Game/LDW/Blueprints/Widgets/WBP_PauseMenu.WBP_PauseMenu_C|GetWBP_InventoryTab (Variables|/Game/LDW/Blueprints/Characters/Player/BP_PlayerControllerGameplay.BP_PlayerControllerGameplay_C|GetPauseMenuWBP _asbp_player_controller_gameplay))))
    (:then_2
      (bind _asbp_game_instance_custom (Utilities|Casting|CastToBP_GameInstanceCustom (Game|GetGameInstance)))
      (Utilities|IsValid (Variables|/Game/LDW/Blueprints/Game/BP_GameInstanceCustom.BP_GameInstanceCustom_C|GetCurrentSaveGame _asbp_game_instance_custom)
        (:Is%20Valid
          (Variables|/Game/LDW/Blueprints/Data/BP_SaveGame.BP_SaveGame_C|SetTotalDeathTimes (Variables|/Game/LDW/Blueprints/Game/BP_GameInstanceCustom.BP_GameInstanceCustom_C|GetCurrentSaveGame _asbp_game_instance_custom) (+ (Variables|/Game/LDW/Blueprints/Data/BP_SaveGame.BP_SaveGame_C|GetTotalDeathTimes (Variables|/Game/LDW/Blueprints/Game/BP_GameInstanceCustom.BP_GameInstanceCustom_C|GetCurrentSaveGame _asbp_game_instance_custom)) 1)))))))

(fn ConstructionScript)

(fn OnEquipmentIndexChanged
  (params (OldType :type EHoldingObjectType%20Enum :default "None") (NewType :type EHoldingObjectType%20Enum :default "None"))
  (Utilities|FlowControl|Sequence
    (:then_0
      (switch Utilities|FlowControl|Switch|SwitchonEHoldingObjectType NewType
        (:None
          (Rendering|Components|Light|SetIntensity (Variables|Default|GetTorchPointLightComp) 0.0 :!label _label))
        (:Torch
          (CallFunction|TorchStartBurning))
        (:GunSword
          (goto _label))))
    (:then_1
      (Class|CharacterPlayerBase|UnderFootDirectionEffect 0.4)
      (bind _as_bp_gameplay_controller (Utilities|GetGameplayController)
        (:Valid
          (Utilities|IsValid (Variables|/Game/LDW/Blueprints/Characters/Player/BP_PlayerControllerGameplay.BP_PlayerControllerGameplay_C|GetPersistentGameplayWBP _as_bp_gameplay_controller)
            (:Is%20Valid
              (Default|SetWeaponSlotState (Variables|/Game/LDW/Blueprints/Characters/Player/BP_PlayerControllerGameplay.BP_PlayerControllerGameplay_C|GetPersistentGameplayWBP _as_bp_gameplay_controller) (Utilities|Enum|Equal(Enum) NewType "Torch")))))))))

(fn PlayCameraShake
  (params (CameraShakeClass :type Camera%20Shake%20Base%20Class%20Reference))
  (Camera|PlayWorldCameraShake CameraShakeClass (Transformation|GetActorLocation) 2e+03 5e+03))

(fn AssistSnappingtoClosetTargetifValid
  (bind _returnvalue (Math|Float|MakeLiteralFloat 2.8e+02))
  (bind _returnvalue_2 (Transformation|GetActorLocation))
  (bind _outactors (Collision|SphereOverlapActors (+ (Transformation|GetActorLocation) (* (Math|Vector|GetForwardVector (Transformation|GetActorRotation)) (Math|Float|MakeLiteralFloat 2.2e+02))) 2e+02 (Utilities|Array|MakeArray "ObjectTypeQuery3" "ObjectTypeQuery2") "/Script/ProjectNo6.CharacterEnemyBase"))
  (Utilities|FlowControl|Sequence
    (:then_0
      (bind _array_element (Utilities|Array|ForEachLoopwithBreak _outactors :!label _label)
        (:LoopBody
          (bind _ascharacter_enemy_base (Utilities|Casting|CastToCharacterEnemyBase _array_element))
          (bind _returnvalue_3 (Class|CustomFunctionLibrary|AngleBetween2Vector (Math|Vector|MakeVector (.x (- (Transformation|GetActorLocation _array_element) (Transformation|GetActorLocation))) (.y (- (Transformation|GetActorLocation _array_element) (Transformation|GetActorLocation))) 0.0) (Math|Vector|GetForwardVector (Transformation|GetActorRotation))))
          (if (< (Math|Float|Absolute(Float) _returnvalue_3) 2e+01)
            (Utilities|FlowControl|Sequence
              (:then_0
                (if (> (Math|Vector|VectorLength (- (Transformation|GetActorLocation _ascharacter_enemy_base) _returnvalue_2)) _returnvalue)
                  (Class|TransformComponent|MovetoLocation (Variables|Default|GetTransformComp) (+ (* (Math|Vector|Normalize (Math|Vector|MakeVector (.x (- _returnvalue_2 (Transformation|GetActorLocation _ascharacter_enemy_base))) (.y (- _returnvalue_2 (Transformation|GetActorLocation _ascharacter_enemy_base))) 0.0)) _returnvalue) (Math|Vector|MakeVector 0.0 0.0 (.z (Transformation|GetActorLocation))) (Math|Vector|MakeVector (.X (Math|Vector|BreakVector (Transformation|GetActorLocation _ascharacter_enemy_base))) (.Y (Math|Vector|BreakVector (Transformation|GetActorLocation _ascharacter_enemy_base))) 0.0)) 0.2 "Linear" true "None")))
              (:then_1
                (goto _label Break)))))))))

(fn GetCameraArmLength
  (return (Variables|/Script/Engine.SpringArmComponent|GetTargetArmLength (Variables|Default|GetMainSpringArmComp))))

(fn SetCameraArmLength
  (params (Length :type Float%20%28double-precision%29))
  (Variables|/Script/Engine.SpringArmComponent|SetTargetArmLength (Variables|Default|GetMainSpringArmComp) Length))