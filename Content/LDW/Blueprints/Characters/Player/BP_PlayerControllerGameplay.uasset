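; Gameplay player controller that owns the HUD and menu widgets and restores the saved story state.
; BeginPlay creates layered widgets, then after a delay uses the save game to start a dialogue or re-grant the current mission.
; Events drive pause, temple objective selection, dialogue and fade transitions, switching input mode and cursor or camera view as needed.
; Hit and coin callbacks update the blood screen, health and coin displays.
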(event Custom|CreateObjectiveWigets
  (bind _templeselectionwbp (Variables|Default|GetTempleSelectionWBP))
  ;[1 1 1] Create Objective Widgets
  (Utilities|IsValid _templeselectionwbp
    (:Is%20Valid
      (Default|CreateRowsOfObjectiveWidgets _templeselectionwbp))))

(event Custom|DisplayDialogue
  (params (DialogueLine :type Dialogue%20Line%20Structure) (LineIndex :type Integer))
  (bind _storywbp (Variables|Default|GetStoryWBP))
  ;[1 1 1] Display Dialogue
  (Default|DisplayDialogue (Variables|/Game/LDW/Blueprints/Widgets/Story/WBP_StoryCanvas.WBP_StoryCanvas_C|GetWBP_Narrator (Variables|Default|GetStoryWBP)) DialogueLine LineIndex)
  (if (== LineIndex 0)
    (Default|SetActivationState _storywbp true)
    (Input|SetInputModeUIOnly self _storywbp "LockAlways")
    (CallFunction|SetCameraView 1)))

(event Custom|SetCameraView
  (params (ViewIndex :type Integer))
  ;[1 1 1] Set Camera View
  (bind _asbp_character_player_human (Utilities|Casting|CastToBP_CharacterPlayerHuman (Pawn|GetControlledPawn)))
  (Default|SetCameraView _asbp_character_player_human ViewIndex))

(event EventBeginPlay
  ;[1 1 1] BeginPlay
  (|CallParentFunction)
  (Utilities|FlowControl|Sequence
    (:then_0
      (bind _returnvalue (UserInterface|CreateWidget "/Game/LDW/Blueprints/Widgets/WBP_PersistentGameplay.WBP_PersistentGameplay_C" self))
      (bind _output_get (Variables|Default|SetPersistentGameplayWBP _returnvalue))
      (UserInterface|Viewport|AddtoViewport _output_get 4)
      (bind _returnvalue_2 (UserInterface|CreateWidget "/Game/LDW/Blueprints/Widgets/WBP_PauseMenu.WBP_PauseMenu_C" self))
      (UserInterface|Viewport|AddtoViewport _returnvalue_2 6)
      (bind _output_get_2 (Variables|Default|SetPauseMenuWBP _returnvalue_2))
      (Widget|SetVisibility _output_get_2 "Collapsed"))
    (:then_1
      (bind _returnvalue_3 (UserInterface|CreateWidget "/Game/LDW/Blueprints/Widgets/WBP_TempleSelection.WBP_TempleSelection_C" self))
      (bind _output_get_3 (Variables|Default|SetTempleSelectionWBP _returnvalue_3))
      (UserInterface|Viewport|AddtoViewport _output_get_3 8)
      (Widget|SetVisibility _output_get_3 "Collapsed")
      (bind _returnvalue_4 (UserInterface|CreateWidget "/Game/LDW/Blueprints/Widgets/WBP_UpgradeSelectionsPanel.WBP_UpgradeSelectionsPanel_C" self))
      (UserInterface|Viewport|AddtoViewport _returnvalue_4 4)
      (Widget|SetVisibility _returnvalue_4 "Collapsed")
      (Variables|Default|SetUpgradeSelectionsPanel _returnvalue_4))
    (:then_2
      (bind _returnvalue_5 (UserInterface|CreateWidget "/Game/LDW/Blueprints/Widgets/WBP_Transition.WBP_Transition_C" self))
      (bind _output_get_4 (Variables|Default|SetTransitionWBP _returnvalue_5))
      (UserInterface|Viewport|AddtoViewport _output_get_4 20)
      (Default|TransitionOutOfBlack _output_get_4)
      (bind _returnvalue_6 (UserInterface|CreateWidget "/Game/LDW/Blueprints/Widgets/WBP_BloodScreen.WBP_BloodScreen_C" self))
      (UserInterface|Viewport|AddtoViewport _returnvalue_6 18)
      (Variables|Default|SetBloodScreenWidget _returnvalue_6))
    (:then_3
      (bind _returnvalue_7 (UserInterface|CreateWidget "/Game/LDW/Blueprints/Widgets/WBP_NPCInteractionCanvas.WBP_NPCInteractionCanvas_C" self))
      (bind _output_get_5 (Variables|Default|SetNPCInteractionWBP _returnvalue_7))
      (UserInterface|Viewport|AddtoViewport _output_get_5 5)
      (bind _returnvalue_8 (UserInterface|CreateWidget "/Game/LDW/Blueprints/Widgets/Story/WBP_StoryCanvas.WBP_StoryCanvas_C" self))
      (UserInterface|Viewport|AddtoViewport _returnvalue_8 10)
      (Variables|Default|SetStoryWBP _returnvalue_8))
    (:then_4
      (Utilities|FlowControl|Delay 1.5)
      (bind _asbp_game_instance_custom (Utilities|Casting|CastToBP_GameInstanceCustom (Game|GetGameInstance)))
      (Utilities|IsValid (Variables|/Game/LDW/Blueprints/Game/BP_GameInstanceCustom.BP_GameInstanceCustom_C|GetCurrentSaveGame _asbp_game_instance_custom)
        (:Is%20Valid
          (if (Math|Boolean|ANDBoolean (== (Variables|/Game/LDW/Blueprints/Data/BP_SaveGame.BP_SaveGame_C|GetTotalDeathTimes (Variables|/Game/LDW/Blueprints/Game/BP_GameInstanceCustom.BP_GameInstanceCustom_C|GetCurrentSaveGame _asbp_game_instance_custom)) 0) (== (Variables|/Game/LDW/Blueprints/Data/BP_SaveGame.BP_SaveGame_C|GetMissionIndex (Variables|/Game/LDW/Blueprints/Game/BP_GameInstanceCustom.BP_GameInstanceCustom_C|GetCurrentSaveGame _asbp_game_instance_custom)) -1) (== (Variables|/Game/LDW/Blueprints/Data/BP_SaveGame.BP_SaveGame_C|GetDialogueIndex (Variables|/Game/LDW/Blueprints/Game/BP_GameInstanceCustom.BP_GameInstanceCustom_C|GetCurrentSaveGame _asbp_game_instance_custom)) -1))
            (Default|StartNewDialogue _asbp_game_instance_custom "/Game/LDW/Blueprints/Mission/BP_DStartNewRun_GrantMission.BP_DStartNewRun_GrantMission_C")
            (else
              (Utilities|FlowControl|Sequence
                (:then_0
                  (if (> (Variables|/Game/LDW/Blueprints/Data/BP_SaveGame.BP_SaveGame_C|GetMissionIndex (Variables|/Game/LDW/Blueprints/Game/BP_GameInstanceCustom.BP_GameInstanceCustom_C|GetCurrentSaveGame _asbp_game_instance_custom)) 0)
                    (Default|GrantPlayerNewMission _asbp_game_instance_custom (Utilities|Select :Index (Variables|/Game/LDW/Blueprints/Data/BP_SaveGame.BP_SaveGame_C|GetMissionIndex (Variables|/Game/LDW/Blueprints/Game/BP_GameInstanceCustom.BP_GameInstanceCustom_C|GetCurrentSaveGame _asbp_game_instance_custom)) :Option%200 0 :Option%201 "/Game/LDW/Blueprints/Mission/BP_MissionStartNewRun.BP_MissionStartNewRun_C" :Option%202 "/Game/LDW/Blueprints/Mission/BP_MissionKillEnemies.BP_MissionKillEnemies_C" :Option%203 "/Game/LDW/Blueprints/Mission/BP_MissionKillBoss.BP_MissionKillBoss_C"))))
                (:then_1
                  (if (and (> (Variables|/Game/LDW/Blueprints/Data/BP_SaveGame.BP_SaveGame_C|GetDialogueIndex (Variables|/Game/LDW/Blueprints/Game/BP_GameInstanceCustom.BP_GameInstanceCustom_C|GetCurrentSaveGame _asbp_game_instance_custom)) 0) (!= (Variables|/Game/LDW/Blueprints/Data/BP_SaveGame.BP_SaveGame_C|GetDialogueIndex (Variables|/Game/LDW/Blueprints/Game/BP_GameInstanceCustom.BP_GameInstanceCustom_C|GetCurrentSaveGame _asbp_game_instance_custom)) 6))
                    (Default|StartNewDialogue _asbp_game_instance_custom (Utilities|Select :Index (Variables|/Game/LDW/Blueprints/Data/BP_SaveGame.BP_SaveGame_C|GetDialogueIndex (Variables|/Game/LDW/Blueprints/Game/BP_GameInstanceCustom.BP_GameInstanceCustom_C|GetCurrentSaveGame _asbp_game_instance_custom)) :Option%200 0 :Option%201 "/Game/LDW/Blueprints/Mission/BP_DStartNewRun_GrantMission.BP_DStartNewRun_GrantMission_C" :Option%202 "/Game/LDW/Blueprints/Mission/BP_DStartNewRun_MissionCompleted.BP_DStartNewRun_MissionCompleted_C" :Option%203 "/Game/LDW/Blueprints/Mission/BP_DKillEnemies_MissionGranting.BP_DKillEnemies_MissionGranting_C" :Option%204 "/Game/LDW/Blueprints/Mission/BP_DKillEnemies_MissionCompletion.BP_DKillEnemies_MissionCompletion_C" :Option%205 "/Game/LDW/Blueprints/Mission/BP_DKillBoss_MissionCompletion.BP_DKillBoss_MissionCompletion_C" :Option%206 0))))))))))))

(event EventTick
  (params (DeltaSeconds :type Float%20%28single-precision%29))
  ;[1 1 1] Tick
  (|CallParentFunction 0.0))

(event EventHandleEscapeTriggered
  (params (Value :type Input%20Action%20Value%20Structure%20%28by%20ref%29))
  (bind _pausemenuwbp (Variables|Default|GetPauseMenuWBP))
  ;[1 1 1] Handle Escape Input Triggered
  (|CallParentFunction Value)
  (Utilities|FlowControl|Sequence
    (:then_0
      (Utilities|IsValid _pausemenuwbp
        (:Is%20Valid
          (Input|SetInputModeUIOnly self _pausemenuwbp "DoNotLock")
          (Variables|Default|SetbShowMouseCursor true)
          (Default|SetState _pausemenuwbp true)
          (Variables|Default|SetbUpdateGameplayMouseLocation false))))))

(event EventBacktoPersistentGameplay
  (bind _persistentgameplaywbp (Variables|Default|GetPersistentGameplayWBP))
  ;[1 1 1] Back To Persistent Gameplay
  (|CallParentFunction)
  (Utilities|IsValid _persistentgameplaywbp
    (:Is%20Valid
      (Input|SetInputModeGameandUI self _persistentgameplaywbp "LockAlways" false)
      (Variables|Default|SetbShowMouseCursor true))))

(event EventTriggerTempleSelection
  (bind _templeselectionwbp (Variables|Default|GetTempleSelectionWBP))
  ;[1 1 1] Trigger Temple Selection
  (|CallParentFunction)
  (Utilities|IsValid _templeselectionwbp
    (:Is%20Valid
      (Default|SetState _templeselectionwbp true)
      (Input|SetInputModeUIOnly self _templeselectionwbp "DoNotLock")
      (Variables|Default|SetbShowMouseCursor true))))

(event EventHandleonCompletedObjectiveDelegate
  (params (ObjectiveIndex :type Integer) (FloorIndex :type Integer) (ObjectiveType :type EFloorObjectiveType%20Enum :default "Empty"))
  (bind _templeselectionwbp (Variables|Default|GetTempleSelectionWBP))
  ;[1 1 1] Handle On Completed Objective Delegate
  (Utilities|IsValid _templeselectionwbp
    (:Is%20Valid
      (Default|ShowObjectivesSelection _templeselectionwbp)
      (Input|SetInputModeUIOnly self _templeselectionwbp "LockAlways")
      (Variables|Default|SetbShowMouseCursor true)
      (Default|CompleteCurrentRow _templeselectionwbp FloorIndex ObjectiveIndex))))

(event EventTransitiontoBlack
  (bind _transitionwbp (Variables|Default|GetTransitionWBP))
  ;[1 1 1] Transition To Black
  (Utilities|IsValid _transitionwbp
    (:Is%20Valid
      (Default|TransitionintoBlack _transitionwbp))))

(event EventTransitionOutOfBlack
  (bind _transitionwbp (Variables|Default|GetTransitionWBP))
  ;[1 1 1] Transition Out Of Black
  (Utilities|IsValid _transitionwbp
    (:Is%20Valid
      (Default|TransitionOutOfBlack _transitionwbp))))

(event EventOnCoinsValueChanged
  (params (ChangeAmount :type Integer) (LastValue :type Integer) (NewValue :type Integer))
  (bind _persistentgameplaywbp (Variables|Default|GetPersistentGameplayWBP))
  ;[1 1 1] On Coins Value Changed
  (if (> ChangeAmount 0)
    (Default|DisplayReceivingCoinsNotification (Variables|/Game/LDW/Blueprints/Widgets/WBP_PersistentGameplay.WBP_PersistentGameplay_C|GetWBP_PCoinsNotificationContainer _persistentgameplaywbp) ChangeAmount)
    (Default|UpdateTextCoins (Variables|/Game/LDW/Blueprints/Widgets/WBP_PersistentGameplay.WBP_PersistentGameplay_C|GetWBP_PersistentBottomLeftBar _persistentgameplaywbp) NewValue)))

(event Input|KeyboardEvents|AnyKey
  (params (Key :type Key%20Structure :default "None"))
  ;[1 1 1] Any Key
  (:Pressed
    (Class|PlayerControllerGameplay|CheckInputKeyinInteractableActors Key)))

(fn ConstructionScript)

(fn HandlePosCompleteObjective
  (Default|UpdateCurrentSelectionRow (Variables|Default|GetTempleSelectionWBP)))

(fn ShowBloodScreen
  (bind _bloodscreenwidget (Variables|Default|GetBloodScreenWidget))
  (Utilities|IsValid _bloodscreenwidget
    (:Is%20Valid
      (Default|ShowBloodScreen _bloodscreenwidget))))

(fn HandleGetHit
  (params (Damage%20Details :type Damage%20Details%20Object%20Reference))
  (if (and (Utilities|IsValid Damage%20Details) (Class|DamageDetails|IsDamageDetailsValid Damage%20Details))
    (CallFunction|ShowBloodScreen)
    (bind _asbp_character_player_human (Utilities|GetControlledPawnasBPHuman)
      (:Valid
        (Default|UpdateHealth (Variables|Default|GetPersistentGameplayWBP) (Class|StatComponent|GetStat (Class|CharacterPlayerBase|GetStatComp _asbp_character_player_human) "HP"))))))

(fn HideBottomLeftInfo
  (Widget|SetVisibility (Variables|/Game/LDW/Blueprints/Widgets/WBP_PersistentGameplay.WBP_PersistentGameplay_C|GetWBP_PersistentBottomLeftBar (Variables|Default|GetPersistentGameplayWBP)) "Hidden"))

(fn ShowBottomLeftInfo
  (Widget|SetVisibility (Variables|/Game/LDW/Blueprints/Widgets/WBP_PersistentGameplay.WBP_PersistentGameplay_C|GetWBP_PersistentBottomLeftBar (Variables|Default|GetPersistentGameplayWBP)) "HitTestInvisible"))