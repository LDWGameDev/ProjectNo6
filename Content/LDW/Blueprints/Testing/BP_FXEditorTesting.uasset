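; BP_FXEditorTesting is a test actor that lays out the level's Cascade and Niagara effects for viewing.
; From BeginPlay it loops on a timed interval, calling ResetFX each time.
; ResetFX destroys emitter actors with duplicate assets, reactivates the first of each, and collects them in one array.
; It then arranges the survivors in a roughly square, evenly spaced grid using the square root of their count.
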(event Custom|ResetFX
  (bind _returnvalue (Math|Float|MakeLiteralFloat 5e+02))
  (bind _self self)
  (bind _cascadeassetarray (Variables|Default|GetCascadeAssetArray))
  (bind _niagaraassetarray (Variables|Default|GetNiagaraAssetArray))
  (Utilities|Array|Clear (Variables|Default|GetCascadeAssetArray))
  (Utilities|Array|Clear (Variables|Default|GetNiagaraAssetArray))
  (Utilities|Array|Clear (Variables|Default|GetFXActorArray))
  (Variables|Default|SetRowIndexCounter 0)
  (Variables|Default|SetColumnIndexCounter 0)
  (bind _outactors (Actor|GetAllActorsOfClass _self "/Script/Engine.Emitter"))
  (for _array_element _outactors
    (if (Utilities|Array|ContainsItem _cascadeassetarray (Effects|Components|ParticleSystem|GetFXSystemAsset (Variables|/Script/Engine.Emitter|GetParticleSystemComponent _array_element)))
      (Actor|DestroyActor _array_element)
      (else
        (Components|Activation|Activate (Variables|/Script/Engine.Emitter|GetParticleSystemComponent _array_element) true)
        (Utilities|Array|Add _cascadeassetarray (Effects|Components|ParticleSystem|GetFXSystemAsset (Variables|/Script/Engine.Emitter|GetParticleSystemComponent _array_element)))
        (Utilities|Array|Add (Variables|Default|GetFXActorArray) _array_element))))
  (bind _outactors_2 (Actor|GetAllActorsOfClass _self "/Script/Niagara.NiagaraActor"))
  (for _array_element_2 _outactors_2
    (if (Utilities|Array|ContainsItem _niagaraassetarray (AssetData|GetAsset (Variables|/Script/Niagara.NiagaraActor|GetNiagaraComponent _array_element_2)))
      (Actor|DestroyActor _array_element_2)
      (else
        (Components|Activation|Activate (Variables|/Script/Niagara.NiagaraActor|GetNiagaraComponent _array_element_2) true)
        (Utilities|Array|Add _niagaraassetarray (AssetData|GetAsset (Variables|/Script/Niagara.NiagaraActor|GetNiagaraComponent _array_element_2)))
        (Utilities|Array|Add (Variables|Default|GetFXActorArray) _array_element_2))))
  (if true
    (for _array_element_3 (Variables|Default|GetFXActorArray)
      (Utilities|IsValid _array_element_3
        (:Is%20Valid
          (Transformation|SetActorLocation _array_element_3 (Math|Vector|MakeVector (* (Variables|Default|GetRowIndexCounter) _returnvalue) (* (Variables|Default|GetColumnIndexCounter) _returnvalue) 0.0) false false)
          (bind _result (Math|Integer|IncrementInt (Variables|Default|GetColumnIndexCounter))
            (:%20%20
              (if (>= _result (Class|KismetMathLibrary|FFloor64 (Math|Float|Sqrt (Math|Conversions|ToFloat(Integer) (Utilities|Array|Length (Variables|Default|GetFXActorArray))))))
                (Variables|Default|SetColumnIndexCounter 0)
                (Math|Integer|IncrementInt (Variables|Default|GetRowIndexCounter))))))))))

(event EventBeginPlay
  (Utilities|FlowControl|Delay self (Variables|Default|GetInterval) :!label _label)
  (CallFunction|ResetFX)
  (goto _label))

(fn ConstructionScript)