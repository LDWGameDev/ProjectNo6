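; Torch holdable equipment Blueprint that shows its mesh only while the torch is held.
; The holding mesh is hidden on BeginPlay, shown on OnStartHolding and hidden again on OnStopHolding, with visibility propagated to child components.
; Both holding events call their parent implementations, and starting to hold also plays a draw-torch sound through a custom spawn-sound call.
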(event EventOnStartHolding
  ;[1 1 1] OnStartHolding
  (|CallParentFunction)
  (Rendering|SetVisibility (Variables|Default|GetHoldingMeshComp) true true)
  (Class|CustomFunctionLibrary|CustomSpawnSoundatLocation "player_draw_torch" "0, 0, 0"))

(event EventOnStopHolding
  ;[1 1 1] OnStopHolding
  (|CallParentFunction)
  (Rendering|SetVisibility (Variables|Default|GetHoldingMeshComp) false true))

(event EventBeginPlay
  ;[1 1 1] BeginPlay
  (Rendering|SetVisibility (Variables|Default|GetHoldingMeshComp) false true))

(fn ConstructionScript)