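; Base Blueprint for mission dialogues that plays an array of lines through the gameplay player controller.
; Starting records the dialogue index in the save game, and each TriggerNextDialogue call displays the next line until none remain.
; Finishing resets the saved index, animates the narrator out, then returns to persistent gameplay after a timer.
; Helpers add coins, show notifications and clear the game instance's current dialogue; the skipped-line event is empty.
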(event Custom|OnFinished
  ;[1 1 1] On Finished
  (CallFunction|SetSaveGameDialogueIndex -1)
  (bind _gameplaypc (Utilities|GetGameplayPlayerController)
    (:Success
      (Default|PlayDisappearAnimation (Variables|/Game/LDW/Blueprints/Widgets/Story/WBP_StoryCanvas.WBP_StoryCanvas_C|GetWBP_Narrator (Variables|/Game/LDW/Blueprints/Characters/Player/BP_PlayerControllerGameplay.BP_PlayerControllerGameplay_C|GetStoryWBP _gameplaypc)))
      (Utilities|Time|SetTimerbyEvent (delegate Custom|DeactivateStoryWBP) 1.25))))

(event Custom|DeactivateStoryWBP
  (Default|SetActivationState (Variables|/Game/LDW/Blueprints/Characters/Player/BP_PlayerControllerGameplay.BP_PlayerControllerGameplay_C|GetStoryWBP (stale Custom|OnFinished _gameplaypc)) false)
  (Default|SetCameraView (stale Custom|OnFinished _gameplaypc))
  (Class|PlayerControllerGameplay|BacktoPersistentGameplay (stale Custom|OnFinished _gameplaypc)))

(event Custom|RemoveFromGameInstanceCurrentDialogue
  ;[1 1 1] Remove From Game Instance Current Dialogue
  (bind _asbp_game_instance_custom (Utilities|Casting|CastToBP_GameInstanceCustom (Class|MissionBase|CustomGetGameInstance)))
  (Variables|/Game/LDW/Blueprints/Game/BP_GameInstanceCustom.BP_GameInstanceCustom_C|SetCurrentDialogue _asbp_game_instance_custom 0))

(event Custom|TriggerNextDialogue
  ;[1 1 1] Trigger Next Dialogue
  (if (< (+ (Variables|Default|GetCurrentIndex) 1) (Utilities|Array|Length (Variables|Default|GetDialogueLines)))
    (bind _output_get (Variables|Default|SetCurrentIndex (+ (Variables|Default|GetCurrentIndex) 1)))
    (bind _gameplaypc (Utilities|GetGameplayPlayerController)
      (:Success
        (Default|DisplayDialogue _gameplaypc (Utilities|Array|Get(acopy) (Variables|Default|GetDialogueLines) _output_get) _output_get)))
    (else
      (CallFunction|OnFinished))))

(event Custom|OnSkippedDialogueLine
  ;[1 1 1] On Skipped Dialogue Line
)

(event EventOnStarted
  ;[1 1 1] On Started
  (Variables|Default|SetCurrentIndex -1)
  (CallFunction|TriggerNextDialogue)
  (CallFunction|SetSaveGameDialogueIndex (Variables|Default|GetDialogueIndex)))

(fn AddCoins
  (params (AmountToAdd :type Integer))
  (bind _returnvalue (Class|MissionBase|CustomGetPlayerController))
  (bind _asbp_player_controller_gameplay (Utilities|Casting|CastToBP_PlayerControllerGameplay _returnvalue))
  (Class|PlayerControllerGameplay|AddtoCoins _asbp_player_controller_gameplay AmountToAdd))

(fn Notify
  (params (Content :type String))
  (bind _returnvalue (Class|MissionBase|CustomGetPlayerController))
  (bind _asbp_player_controller_gameplay (Utilities|Casting|CastToBP_PlayerControllerGameplay _returnvalue))
  (Default|Notify (Variables|/Game/LDW/Blueprints/Characters/Player/BP_PlayerControllerGameplay.BP_PlayerControllerGameplay_C|GetPersistentGameplayWBP _asbp_player_controller_gameplay) Content))

(fn SetSaveGameDialogueIndex
  (params (DialogueIndex :type Integer))
  (bind _asbp_game_instance_custom (Utilities|Casting|CastToBP_GameInstanceCustom (Class|MissionBase|CustomGetGameInstance)))
  (Utilities|IsValid (Variables|/Game/LDW/Blueprints/Game/BP_GameInstanceCustom.BP_GameInstanceCustom_C|GetCurrentSaveGame _asbp_game_instance_custom)
    (:Is%20Valid
      (Variables|/Game/LDW/Blueprints/Data/BP_SaveGame.BP_SaveGame_C|SetDialogueIndex (Variables|/Game/LDW/Blueprints/Game/BP_GameInstanceCustom.BP_GameInstanceCustom_C|GetCurrentSaveGame _asbp_game_instance_custom) DialogueIndex))))