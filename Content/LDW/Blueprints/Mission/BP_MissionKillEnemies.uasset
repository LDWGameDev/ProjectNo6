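; Kill-enemies mission that requires a set number of kills from configured enemy classes, then rewards coins.
; On start it binds to the game instance's enemy-died and floor-completed delegates, counting matching kills and updating the mission widget.
; Reaching the target unbinds kill tracking, but completion waits for a floor-completed event, which triggers a dialogue and delayed finish.
; Finishing pays out, removes the widget and, after a delay, leaves the ongoing missions list.
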(event Custom|HandleOnEnemyDiedDelegate
  (params (EnemyClass :type Actor%20Class%20Reference))
  (bind _missionwidget (Variables|Default|GetMissionWidget))
  (if (CallFunction|IsValidEnemyTypes EnemyClass)
    (bind _result (Math|Integer|IncrementInt (Variables|Default|GetNumberKilled))
      (:%20%20
        (if (>= _result (Variables|Default|GetNumberToKill))
          (bind _asbp_game_instance_custom (Utilities|Casting|CastToBP_GameInstanceCustom (Class|Mission|CustomGetGameInstance)))
          (EventDispatchers|UnbindEventfromOnEnemyDiedDelegate _asbp_game_instance_custom (delegate Custom|HandleOnEnemyDiedDelegate))
          (if (and (Utilities|IsValid _missionwidget) (Utilities|DoesObjectImplementInterface _missionwidget "/Game/LDW/Blueprints/Widgets/Story/BPI_WidgetInterface.BPI_WidgetInterface_C"))
            (Class|BPIWidgetInterface|MissionSetCompleteState(Message) _missionwidget false)
            (bind _aswbp_persistent_kill_enemies_mission (Utilities|Casting|CastToWBP_PersistentKillEnemiesMission (Variables|Default|GetMissionWidget)))
            (Default|UpdateKillsCount _aswbp_persistent_kill_enemies_mission (Variables|Default|GetNumberToKill) (Variables|Default|GetNumberKilled)))
          (else
            (bind _aswbp_persistent_kill_enemies_mission_2 (Utilities|Casting|CastToWBP_PersistentKillEnemiesMission (Variables|Default|GetMissionWidget)))
            (Default|UpdateKillsCount _aswbp_persistent_kill_enemies_mission_2 (Variables|Default|GetNumberToKill) (Variables|Default|GetNumberKilled))))))))

(event Custom|CheckMissionCompletion
  (if (>= (Variables|Default|GetNumberKilled) (Variables|Default|GetNumberToKill))
    (EventDispatchers|UnbindEventfromOnCompletedFloor (stale EventOnStarted _asbp_game_instance_custom) (delegate Custom|CheckMissionCompletion))
    (bind _asbp_game_instance_custom (Utilities|Casting|CastToBP_GameInstanceCustom (Class|Mission|CustomGetGameInstance)))
    (Default|StartNewDialogue _asbp_game_instance_custom "/Game/LDW/Blueprints/Mission/BP_DKillEnemies_MissionCompletion.BP_DKillEnemies_MissionCompletion_C")
    (Utilities|Time|SetTimerbyEvent (delegate Custom|SelfFinish) 1.0)))

(event Custom|SelfFinish
  (CallFunction|OnFinished))

(event Custom|SelfRemoveFromOnGoing
  (CallFunction|RemovefromonGoingMissions))

(event EventOnStarted
  ;[1 1 1] On Started
  (|CallParentFunction)
  (bind _asbp_game_instance_custom (Utilities|Casting|CastToBP_GameInstanceCustom (Class|Mission|CustomGetGameInstance)))
  (EventDispatchers|AssignOnEnemyDiedDelegate _asbp_game_instance_custom (delegate Custom|HandleOnEnemyDiedDelegate))
  (Variables|Default|SetNumberKilled 0)
  (EventDispatchers|BindEventtoOnCompletedFloor _asbp_game_instance_custom (delegate Custom|CheckMissionCompletion)))

(event EventOnFinished
  (bind _missionwidget (Variables|Default|GetMissionWidget))
  ;[1 1 1] On Finished
  (|CallParentFunction)
  (Utilities|FlowControl|Sequence
    (:then_0
      (CallFunction|AddCoins 45)
      (Utilities|IsValid _missionwidget
        (:Is%20Valid
          (Widget|RemovefromParent _missionwidget))))
    (:then_1
      (Utilities|Time|SetTimerbyEvent (delegate Custom|SelfRemoveFromOnGoing) 1.0))))

(fn IsValidEnemyTypes
  (params (EnemyClass :type Actor%20Class%20Reference))
  (for _array_element (Variables|Default|GetEnemyTypes)
    (if (Utilities|ClassIsChildOf EnemyClass _array_element)
      (return true)))
  (return false))

(fn GetPersistentDescription
  (return (Utilities|String|Append "Kill " (Utilities|String|ToString(Integer) (Variables|Default|GetNumberToKill)) " enemies of any types")))