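; Base Blueprint for missions, handling start and finish notifications, save progress and shared helper functions.
; On start it shows the mission name on the player controller's persistent gameplay widget and writes its index to the current save game; on finish it notifies and resets that index to -1.
; Helpers add coins through the player controller and remove the mission from the game instance's ongoing list, while GetPersistentDescription returns an empty string.
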(event Custom|OnStarted
  ;[1 1 1] On Started
  (CallFunction|Notify (Utilities|String|Append "New Mission" " 
" (Variables|Default|GetMissionName)))
  (CallFunction|SetSaveGameMissionIndex (Variables|Default|GetMissionIndex)))

(event Custom|OnFinished
  ;[1 1 1] On Finished
  (CallFunction|Notify (Utilities|String|Append "Mission Completed" " 
" (Variables|Default|GetMissionName)))
  (CallFunction|SetSaveGameMissionIndex -1))

(fn GetPersistentDescription
  (return ""))

(fn RemovefromonGoingMissions
  (bind _asbp_game_instance_custom (Utilities|Casting|CastToBP_GameInstanceCustom (Class|Mission|CustomGetGameInstance)))
  (Default|RemoveonGoingMission _asbp_game_instance_custom self))

(fn Notify
  (params (Content :type String))
  (bind _returnvalue (Class|Mission|CustomGetPlayerController))
  (bind _asbp_player_controller_gameplay (Utilities|Casting|CastToBP_PlayerControllerGameplay _returnvalue))
  (Default|Notify (Variables|/Game/LDW/Blueprints/Characters/Player/BP_PlayerControllerGameplay.BP_PlayerControllerGameplay_C|GetPersistentGameplayWBP _asbp_player_controller_gameplay) Content))

(fn AddCoins
  (params (AmountToAdd :type Integer))
  (bind _returnvalue (Class|Mission|CustomGetPlayerController))
  (bind _asbp_player_controller_gameplay (Utilities|Casting|CastToBP_PlayerControllerGameplay _returnvalue))
  (Class|PlayerControllerGameplay|AddtoCoins _asbp_player_controller_gameplay AmountToAdd))

(fn SetSaveGameMissionIndex
  (params (MissionIndex :type Integer))
  (bind _asbp_game_instance_custom (Utilities|Casting|CastToBP_GameInstanceCustom (Class|Mission|CustomGetGameInstance)))
  (Utilities|IsValid (Variables|/Game/LDW/Blueprints/Game/BP_GameInstanceCustom.BP_GameInstanceCustom_C|GetCurrentSaveGame _asbp_game_instance_custom)
    (:Is%20Valid
      (Variables|/Game/LDW/Blueprints/Data/BP_SaveGame.BP_SaveGame_C|SetMissionIndex (Variables|/Game/LDW/Blueprints/Game/BP_GameInstanceCustom.BP_GameInstanceCustom_C|GetCurrentSaveGame _asbp_game_instance_custom) MissionIndex))))