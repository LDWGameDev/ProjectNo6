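; Mission Blueprint for killing the boss, Master Grunt, on the final floor.
; On start it binds to the custom game instance's enemy-died delegate and waits for a BP_GruntMaster death, then unbinds.
; Chained timers then start the completion dialogue and, shortly after, finish the mission.
; Finishing calls the parent logic and saves the new mission index.
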(event Custom|HandleOnEnemyDiedDelegate
  (params (EnemyClass :type Actor%20Class%20Reference))
  (if (== EnemyClass "/Game/LDW/Blueprints/Characters/Enemies/MasterGrunt/BP_GruntMaster.BP_GruntMaster_C")
    (EventDispatchers|UnbindEventfromOnEnemyDiedDelegate (stale EventOnStarted _asbp_game_instance_custom) (delegate Custom|HandleOnEnemyDiedDelegate))
    (Utilities|Time|SetTimerbyEvent (delegate Custom|DisplayKillBossDialogue) 6.0)))

(event Custom|DisplayKillBossDialogue
  (bind _asbp_game_instance_custom (Utilities|Casting|CastToBP_GameInstanceCustom (Class|Mission|CustomGetGameInstance)))
  (Default|StartNewDialogue _asbp_game_instance_custom "/Game/LDW/Blueprints/Mission/BP_DKillBoss_MissionCompletion.BP_DKillBoss_MissionCompletion_C")
  (Utilities|Time|SetTimerbyEvent (delegate Custom|SelfFinish) 1.0))

(event Custom|SelfFinish
  (CallFunction|OnFinished))

(event EventOnStarted
  ;[1 1 1] On Started
  (|CallParentFunction)
  (bind _asbp_game_instance_custom (Utilities|Casting|CastToBP_GameInstanceCustom (Class|Mission|CustomGetGameInstance)))
  (EventDispatchers|BindEventtoOnEnemyDiedDelegate _asbp_game_instance_custom (delegate Custom|HandleOnEnemyDiedDelegate)))

(event EventOnFinished
  ;[1 1 1] On Finished
  (|CallParentFunction)
  (CallFunction|SetSaveGameMissionIndex 10))

(fn GetPersistentDescription
  (return "Kill the boss, Master Grunt, on the final floor"))