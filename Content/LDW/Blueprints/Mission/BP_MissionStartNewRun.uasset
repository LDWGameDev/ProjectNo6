(event Custom|HandleOnStartedNewRunDelegate)

(event Custom|HandleOnStreamLevelLoaded
  (Utilities|Time|SetTimerbyEvent (delegate Custom|DelayFinishMission) 1.0))

(event Custom|DelayFinishMission
  (CallFunction|OnFinished)
  (EventDispatchers|UnbindEventfromOnStreamLevelLoaded (stale EventOnStarted _asbp_game_instance_custom) (delegate Custom|HandleOnStreamLevelLoaded)))

(event Custom|RemoveSelfFromOnGoingMissions
  (CallFunction|RemovefromonGoingMissions))

(event Custom|StartNewRunCompletedMissionDialogue
  (bind _asbp_game_instance_custom (Utilities|Casting|CastToBP_GameInstanceCustom (Class|Mission|CustomGetGameInstance)))
  (Default|StartNewDialogue _asbp_game_instance_custom "/Game/LDW/Blueprints/Mission/BP_DStartNewRun_MissionCompleted.BP_DStartNewRun_MissionCompleted_C"))

(event EventOnStarted
  ;[1 1 1] On Started
  (|CallParentFunction)
  (bind _asbp_game_instance_custom (Utilities|Casting|CastToBP_GameInstanceCustom (Class|Mission|CustomGetGameInstance)))
  (EventDispatchers|AssignOnStartedNewRunDelegate _asbp_game_instance_custom (delegate Custom|HandleOnStartedNewRunDelegate))
  (EventDispatchers|AssignOnStreamLevelLoaded _asbp_game_instance_custom (delegate Custom|HandleOnStreamLevelLoaded)))

(event EventOnFinished
  (bind _missionwidget (Variables|Default|GetMissionWidget))
  ;[1 1 1] On Finished
  (|CallParentFunction)
  (Utilities|FlowControl|Sequence
    (:then_0
      (if (and (Utilities|IsValid _missionwidget) (Utilities|DoesObjectImplementInterface _missionwidget "/Game/LDW/Blueprints/Widgets/Story/BPI_WidgetInterface.BPI_WidgetInterface_C"))
        (Class|BPIWidgetInterface|MissionSetCompleteState(Message) _missionwidget true)
        (CallFunction|AddCoins 30)))
    (:then_1
      (Utilities|Time|SetTimerbyEvent (delegate Custom|RemoveSelfFromOnGoingMissions) 2.0)
      (Utilities|Time|SetTimerbyEvent (delegate Custom|StartNewRunCompletedMissionDialogue) 0.5))))

(fn GetPersistentDescription
  (return "Start your first run"))