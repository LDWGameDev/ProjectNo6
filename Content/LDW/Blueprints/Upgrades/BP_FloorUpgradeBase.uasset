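; BP_FloorUpgradeBase is a base Blueprint for purchasable floor upgrades.
; TakeEffect finds the controller's controlled pawn, casts it to BP_CharacterPlayerHuman, adds itself to that character's FloorUpgradesArray and deducts Price from the controller's coins.
; A GetCharacterHuman helper exposes Success and Failed outputs, so nothing is applied or charged when the cast fails.
; StopEffect is left empty.
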(event Custom|TakeEffect
  (params (GameplayController :type BP%20Player%20Controller%20Gameplay%20Object%20Reference))
  (bind _as_character_human (Utilities|GetCharacterHuman GameplayController)
    (:Success
      (Utilities|Array|Add (Variables|/Game/LDW/Blueprints/Characters/Player/BP_CharacterPlayerHuman.BP_CharacterPlayerHuman_C|GetFloorUpgradesArray _as_character_human) self)
      (Class|PlayerControllerGameplay|AddtoCoins GameplayController (* (Variables|Default|GetPrice) -1)))))

(event Custom|StopEffect
  (params (GameplayController :type BP%20Player%20Controller%20Gameplay%20Object%20Reference)))