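; Upgrade that cuts the human player's stamina points in exchange for a combat bonus.
; DoUpgrade reaches the pawn through the triggering gameplay controller, caps the Power stat at a fixed four and updates the persistent stamina widget's gems to match.
; TypeId then selects one of three 30% bonuses: higher ATK, more damage dealt or less damage taken.
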(event EventDoUpgrade
  (params (PlayerControllerTriggerUpgrading :type Player%20Controller%20Object%20Reference))
  (bind _asbp_player_controller_gameplay (Utilities|Casting|CastToBP_PlayerControllerGameplay PlayerControllerTriggerUpgrading))
  (bind _asbp_character_player_human (Utilities|Casting|CastToBP_CharacterPlayerHuman (Pawn|GetControlledPawn _asbp_player_controller_gameplay)))
  (Utilities|IsValid (Class|CharacterPlayerBase|GetStatComp _asbp_character_player_human)
    (:Is%20Valid
      (Utilities|IsValid (Class|StatComponent|GetStat (Class|CharacterPlayerBase|GetStatComp _asbp_character_player_human) "Power")
        (:Is%20Valid
          (Class|StatBase|SetMinMaxValue (Class|StatComponent|GetStat (Class|CharacterPlayerBase|GetStatComp _asbp_character_player_human) "Power") 0 4)
          (bind _aswbp_persistent_stamina (Utilities|Casting|CastToWBP_PersistentStamina (UserInterface|GetWidget (Class|CharacterPlayerBase|GetPersistentStaminaWidgetComp _asbp_character_player_human))))
          (Default|UpdateStaminaGemsNumber _aswbp_persistent_stamina 4)
          (switch int (Variables|Default|GetTypeId)
            (:0
              ;[1 1 1] Increase Attack By 30%
              (Utilities|IsValid (Class|StatComponent|GetStat (Class|CharacterPlayerBase|GetStatComp _asbp_character_player_human) "ATK")
                (:Is%20Valid
                  (Class|StatBase|SetCurrentValue (Class|StatComponent|GetStat (Class|CharacterPlayerBase|GetStatComp _asbp_character_player_human) "ATK") (Math|Float|Round (* (Math|Conversions|ToFloat(Integer) (Class|StatBase|GetValue (Class|StatComponent|GetStat (Class|CharacterPlayerBase|GetStatComp _asbp_character_player_human) "ATK"))) 1.3)) true))))
            (:1
              ;[1 1 1] Deal More 30% Damage
              (Utilities|IsValid (Class|CharacterPlayerBase|GetCombatComp _asbp_character_player_human)
                (:Is%20Valid
                  (Variables|/Script/ProjectNo6.CombatComponent|SetDealMoreDamageBoost (Class|CharacterPlayerBase|GetCombatComp _asbp_character_player_human) (+ (Variables|/Script/ProjectNo6.CombatComponent|GetDealMoreDamageBoost (Class|CharacterPlayerBase|GetCombatComp _asbp_character_player_human)) 3e+01)))))
            (:2
              ;[1 1 1] Take Less 30% Damage
              (Utilities|IsValid (Class|CharacterPlayerBase|GetCombatComp _asbp_character_player_human)
                (:Is%20Valid
                  (Variables|/Script/ProjectNo6.CombatComponent|SetTakeMoreDamageBoost (Class|CharacterPlayerBase|GetCombatComp _asbp_character_player_human) (- (Variables|/Script/ProjectNo6.CombatComponent|GetTakeMoreDamageBoost (Class|CharacterPlayerBase|GetCombatComp _asbp_character_player_human)) 3e+01)))))))))))