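; An upgrade Blueprint that trades survivability for offense on the human player character.
; When DoUpgrade fires, it casts the triggering controller's pawn to BP_CharacterPlayerHuman and checks that its combat component is valid.
; It then adds configurable boost values to that component's take-more and deal-more damage boosts, so repeated upgrades accumulate.
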(event EventDoUpgrade
  (params (PlayerControllerTriggerUpgrading :type Player%20Controller%20Object%20Reference))
  (bind _asbp_character_player_human (Utilities|Casting|CastToBP_CharacterPlayerHuman (Pawn|GetControlledPawn PlayerControllerTriggerUpgrading)))
  (Utilities|IsValid (Class|CharacterPlayerBase|GetCombatComp _asbp_character_player_human)
    (:Is%20Valid
      (Variables|/Script/ProjectNo6.CombatComponent|SetTakeMoreDamageBoost (Class|CharacterPlayerBase|GetCombatComp _asbp_character_player_human) (+ (Variables|/Script/ProjectNo6.CombatComponent|GetTakeMoreDamageBoost (Class|CharacterPlayerBase|GetCombatComp _asbp_character_player_human)) (Variables|Default|GetTakeMoreBoostValue)))
      (Variables|/Script/ProjectNo6.CombatComponent|SetDealMoreDamageBoost (Class|CharacterPlayerBase|GetCombatComp _asbp_character_player_human) (+ (Variables|/Script/ProjectNo6.CombatComponent|GetDealMoreDamageBoost (Class|CharacterPlayerBase|GetCombatComp _asbp_character_player_human)) (Variables|Default|GetDealMoreBoostValue))))))