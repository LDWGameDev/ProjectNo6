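; BP_FU_IncreaseStamina is an upgrade effect that raises the human player character's maximum Power stat by one.
; TakeEffect casts the controller's pawn to BP_CharacterPlayerHuman through a GetCharacterHuman helper, then updates the stat's range on its stat component.
; StopEffect calls its parent and looks up the character but does not revert the increase.
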(event EventTakeEffect
  (params (GameplayController :type BP%20Player%20Controller%20Gameplay%20Object%20Reference))
  (|CallParentFunction GameplayController)
  (Utilities|IsValid GameplayController
    (:Is%20Valid
      (bind _as_character_human (Utilities|GetCharacterHuman GameplayController)
        (:Success
          (Class|StatBase|SetMinMaxValue (Class|StatComponent|GetStat (Class|CharacterPlayerBase|GetStatComp _as_character_human) "Power") 0 (+ (Variables|/Script/ProjectNo6.StatBase|GetMaxValue (Class|StatComponent|GetStat (Class|CharacterPlayerBase|GetStatComp _as_character_human) "Power")) 1)))))))

(event EventStopEffect
  (params (GameplayController :type BP%20Player%20Controller%20Gameplay%20Object%20Reference))
  (|CallParentFunction GameplayController)
  (Utilities|IsValid GameplayController
    (:Is%20Valid
      (Utilities|GetCharacterHuman GameplayController))))