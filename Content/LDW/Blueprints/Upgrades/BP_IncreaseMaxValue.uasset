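; Upgrade Blueprint that raises the max value of a chosen stat on the player's human character.
; DoUpgrade gets the stat from the controlled pawn's stat component, raises its maximum by a flat or percentage Amount, then adds to its current value.
; In percentage mode, that addition is recalculated from the already raised maximum.
; GetMoreDescription builds the upgrade text from stat type, amount and mode.
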(event EventDoUpgrade
  (params (PlayerControllerTriggerUpgrading :type Player%20Controller%20Object%20Reference))
  (bind _amount (Variables|Default|GetAmount))
  (bind _asbp_player_controller_gameplay (Utilities|Casting|CastToBP_PlayerControllerGameplay PlayerControllerTriggerUpgrading))
  (bind _asbp_character_player_human (Utilities|Casting|CastToBP_CharacterPlayerHuman (Pawn|GetControlledPawn _asbp_player_controller_gameplay)))
  (Utilities|IsValid (Class|CharacterPlayerBase|GetStatComp _asbp_character_player_human)
    (:Is%20Valid
      (Utilities|IsValid (Class|StatComponent|GetStat (Class|CharacterPlayerBase|GetStatComp _asbp_character_player_human) (Variables|Default|GetStatType))
        (:Is%20Valid
          (if (Variables|Default|GetbIsFlatValue)
            (Class|StatBase|SetMinMaxValue (Class|StatComponent|GetStat (Class|CharacterPlayerBase|GetStatComp _asbp_character_player_human) (Variables|Default|GetStatType)) (Variables|/Script/ProjectNo6.StatBase|GetMinValue (Class|StatComponent|GetStat (Class|CharacterPlayerBase|GetStatComp _asbp_character_player_human) (Variables|Default|GetStatType))) (+ (Variables|/Script/ProjectNo6.StatBase|GetMaxValue (Class|StatComponent|GetStat (Class|CharacterPlayerBase|GetStatComp _asbp_character_player_human) (Variables|Default|GetStatType))) _amount))
            (Class|StatBase|AddValue (Class|StatComponent|GetStat (Class|CharacterPlayerBase|GetStatComp _asbp_character_player_human) (Variables|Default|GetStatType)) _amount)
            (else
              (Class|StatBase|SetMinMaxValue (Class|StatComponent|GetStat (Class|CharacterPlayerBase|GetStatComp _asbp_character_player_human) (Variables|Default|GetStatType)) (Variables|/Script/ProjectNo6.StatBase|GetMinValue (Class|StatComponent|GetStat (Class|CharacterPlayerBase|GetStatComp _asbp_character_player_human) (Variables|Default|GetStatType))) (+ (Variables|/Script/ProjectNo6.StatBase|GetMaxValue (Class|StatComponent|GetStat (Class|CharacterPlayerBase|GetStatComp _asbp_character_player_human) (Variables|Default|GetStatType))) (Math|Float|Round (* (Math|Float|SafeDivide (Math|Conversions|ToFloat(Integer) (Variables|Default|GetAmount)) 1e+02) (Math|Conversions|ToFloat(Integer) (Variables|/Script/ProjectNo6.StatBase|GetMaxValue (Class|StatComponent|GetStat (Class|CharacterPlayerBase|GetStatComp _asbp_character_player_human) (Variables|Default|GetStatType))))))))
              (Class|StatBase|AddValue (Class|StatComponent|GetStat (Class|CharacterPlayerBase|GetStatComp _asbp_character_player_human) (Variables|Default|GetStatType)) (Math|Float|Round (* (Math|Float|SafeDivide (Math|Conversions|ToFloat(Integer) (Variables|Default|GetAmount)) 1e+02) (Math|Conversions|ToFloat(Integer) (Variables|/Script/ProjectNo6.StatBase|GetMaxValue (Class|StatComponent|GetStat (Class|CharacterPlayerBase|GetStatComp _asbp_character_player_human) (Variables|Default|GetStatType))))))))))))))

(fn GetMoreDescription
  (return (Utilities|Text|FormatText "{0} by {1}. {2}" (Utilities|Select :Index (Variables|Default|GetStatType) :None "" :HP "Restore health points" :ATK "Increase attack points" :DEF "Increase defense points" :Power "") (Utilities|String|Append (Utilities|String|ToString(Integer) (Variables|Default|GetAmount)) (Utilities|String|SelectString "" " %" (Variables|Default|GetbIsFlatValue))) (Utilities|String|SelectString "" "This percentage value will not affect future increments." (Variables|Default|GetbIsFlatValue)))))