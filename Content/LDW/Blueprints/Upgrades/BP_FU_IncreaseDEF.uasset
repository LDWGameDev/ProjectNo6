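; BP_FU_IncreaseDEF is an upgrade that raises the human player character's DEF stat by a fixed amount while in effect.
; TakeEffect runs the parent logic, then finds the controller's pawn as BP_CharacterPlayerHuman and adds to DEF through its stat component.
; StopEffect reverses this by adding the same negative amount, without calling the parent.
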(event EventStopEffect
  (params (GameplayController :type BP%20Player%20Controller%20Gameplay%20Object%20Reference))
  (Utilities|IsValid GameplayController
    (:Is%20Valid
      (bind _asbp_character_player_human (Utilities|Casting|CastToBP_CharacterPlayerHuman (Pawn|GetControlledPawn GameplayController)))
      (Class|StatBase|AddValue (Class|StatComponent|GetStat (Class|CharacterPlayerBase|GetStatComp _asbp_character_player_human) "DEF") -3))))

(event EventTakeEffect
  (params (GameplayController :type BP%20Player%20Controller%20Gameplay%20Object%20Reference))
  (|CallParentFunction GameplayController)
  (Utilities|IsValid GameplayController
    (:Is%20Valid
      (bind _asbp_character_player_human (Utilities|Casting|CastToBP_CharacterPlayerHuman (Pawn|GetControlledPawn GameplayController)))
      (Class|StatBase|AddValue (Class|StatComponent|GetStat (Class|CharacterPlayerBase|GetStatComp _asbp_character_player_human) "DEF") 3))))