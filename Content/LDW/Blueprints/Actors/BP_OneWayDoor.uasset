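; BP_OneWayDoor is a barrier actor that closes once behind the human player character, with sound, dust, camera shake and background music.
; Until it closes, a camera box sets the camera arm to a longer length on entry and restores the default on exit through a timeline lerp.
; Any of three closing boxes triggers the one-time close for tagged components, resetting the camera and animating the wooden barrier by timeline.
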(event OnComponentBeginOverlap(CameraBox)
  (params (OverlappedComponent :type Primitive%20Component%20Object%20Reference) (OtherActor :type Actor%20Object%20Reference) (OtherComp :type Primitive%20Component%20Object%20Reference) (OtherBodyIndex :type Integer) (bFromSweep :type Boolean) (SweepResult :type Hit%20Result%20Structure%20%28by%20ref%29))
  (bind _asbp_character_player_human (Utilities|Casting|CastToBP_CharacterPlayerHuman OtherActor))
  (if (not (Variables|Default|GetbHasClosed))
    (CallFunction|ChangeCameraLength 1.6e+03 0.5 _asbp_character_player_human)))

(event OnComponentEndOverlap(CameraBox)
  (params (OverlappedComponent :type Primitive%20Component%20Object%20Reference) (OtherActor :type Actor%20Object%20Reference) (OtherComp :type Primitive%20Component%20Object%20Reference) (OtherBodyIndex :type Integer))
  (bind _asbp_character_player_human (Utilities|Casting|CastToBP_CharacterPlayerHuman OtherActor))
  (if (not (Variables|Default|GetbHasClosed))
    (CallFunction|ChangeCameraLength (Variables|/Script/ProjectNo6.CharacterPlayerBase|GetDefaultCameraLength _asbp_character_player_human) 0.5 _asbp_character_player_human)))

(event OnComponentBeginOverlap(DoorClosingBox)
  (params (OverlappedComponent :type Primitive%20Component%20Object%20Reference) (OtherActor :type Actor%20Object%20Reference) (OtherComp :type Primitive%20Component%20Object%20Reference) (OtherBodyIndex :type Integer) (bFromSweep :type Boolean) (SweepResult :type Hit%20Result%20Structure%20%28by%20ref%29))
  (CallFunction|CloseBarrier OtherActor OtherComp))

(event OnComponentBeginOverlap(DoorClosingBox1)
  (params (OverlappedComponent :type Primitive%20Component%20Object%20Reference) (OtherActor :type Actor%20Object%20Reference) (OtherComp :type Primitive%20Component%20Object%20Reference) (OtherBodyIndex :type Integer) (bFromSweep :type Boolean) (SweepResult :type Hit%20Result%20Structure%20%28by%20ref%29))
  (CallFunction|CloseBarrier OtherActor OtherComp))

(event OnComponentBeginOverlap(DoorClosingBox2)
  (params (OverlappedComponent :type Primitive%20Component%20Object%20Reference) (OtherActor :type Actor%20Object%20Reference) (OtherComp :type Primitive%20Component%20Object%20Reference) (OtherBodyIndex :type Integer) (bFromSweep :type Boolean) (SweepResult :type Hit%20Result%20Structure%20%28by%20ref%29))
  (CallFunction|CloseBarrier OtherActor OtherComp))

(event Custom|ChangeCameraLength
  (params (TargetLength :type Float%20%28double-precision%29) (Duration :type Float%20%28double-precision%29) (PlayerHumanCharacter :type BP%20Character%20Player%20Human%20Object%20Reference))
  ;[1 1 1] Change Camera Length
  (Utilities|IsValid PlayerHumanCharacter
    (:Is%20Valid
      (Variables|Default|SetPlayerHumanCharacter PlayerHumanCharacter)
      (Components|Timeline|SetPlayRate (Variables|Default|GetUpdateCameraLengthTimeline) (Math|Float|SafeDivide 1.0 Duration))
      (Variables|Default|SetSavedCameraLength (Default|GetCameraArmLength PlayerHumanCharacter))
      (Variables|Default|SetTargetCameraLength TargetLength)
      (bind _alpha (Timeline|UpdateCameraLengthTimeline PlayFromStart)
        (:Update
          (Utilities|IsValid (Variables|Default|GetPlayerHumanCharacter)
            (:Is%20Valid
              (Default|SetCameraArmLength (Variables|Default|GetPlayerHumanCharacter) (Math|Float|Lerp (Variables|Default|GetSavedCameraLength) (Variables|Default|GetTargetCameraLength) _alpha)))))))))

(event Custom|CloseBarrier
  (params (TriggeringActor :type Actor%20Object%20Reference) (OverlappingComp :type Actor%20Component%20Object%20Reference))
  ;[1 1 1] Close Barrier
  (if (and (Utilities|IsValid OverlappingComp) (Components|ComponentHasTag OverlappingComp "CharacterOverlapping"))
    (bind _asbp_character_player_human (Utilities|Casting|CastToBP_CharacterPlayerHuman TriggeringActor))
    (if (not (Variables|Default|GetbHasClosed))
      (Variables|Default|SetbHasClosed true)
      (Utilities|FlowControl|Sequence
        (:then_0
          (CallFunction|ChangeCameraLength (Variables|/Script/ProjectNo6.CharacterPlayerBase|GetDefaultCameraLength _asbp_character_player_human) 0.5 _asbp_character_player_human)
          (Audio|PlaySound2D "/Game/LDW/Assets/Sounds/S_RockTombStart2.S_RockTombStart2" 1.0 1.0 0.0 0 0))
        (:then_1
          (bind _relative_location (Timeline|DoorClosingTimeline PlayFromStart)
            (:Update
              (Transformation|SetRelativeLocation (Variables|Default|GetWoodenBarrier) _relative_location false false))
            (:Finished
              (Components|Activation|Activate (Variables|Default|GetDust) true)
              (Audio|PlaySound2D "/Game/LDW/Assets/Sounds/S_RockTombImpact.S_RockTombImpact" 1.0 1.0 0.0 0 0)
              (Camera|PlayWorldCameraShake "/Game/LDW/Blueprints/Data/CameraShake/CS_MediumShake.CS_MediumShake_C" (Transformation|GetActorLocation) 3e+03 5e+03)
              (bind _asbp_game_instance_custom (Utilities|Casting|CastToBP_GameInstanceCustom (Game|GetGameInstance)))
              (Default|PlayBGMusic _asbp_game_instance_custom true))))))))

(fn ConstructionScript)