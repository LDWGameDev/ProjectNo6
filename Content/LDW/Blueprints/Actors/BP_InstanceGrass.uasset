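; BP_InstanceGrass is a placeable actor that scatters randomly varied instances of a grass mesh around its location.
; The construction script assigns GrassMesh to an InstancedStaticMesh and adds a random count of world-space instances within the Sphere component's radius.
; Each gets a random yaw, uniform scale and horizontal offset, which biases density toward the centre.
; Randomness is unseeded, so the layout changes whenever construction reruns.
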(event EventBeginPlay)

(fn ConstructionScript
  (bind _sphere (Variables|Default|GetSphere))
  (bind _scalerange (Variables|Config|GetScaleRange))
  (bind _numberofinstancesrange (Variables|Config|GetNumberOfInstancesRange))
  (bind _grassmesh (Variables|Config|GetGrassMesh))
  (bind _returnvalue (Components|Sphere|GetScaledSphereRadius _sphere))
  (Utilities|IsValid _grassmesh
    (:Is%20Valid
      (Components|StaticMesh|SetStaticMesh (Variables|Default|GetInstancedStaticMesh) _grassmesh)
      (bind _output_get (LocalVariables|SetNumberOfInstances (Math|Random|RandomIntegerinRange (Math|Float|Round (.x _numberofinstancesrange)) (Math|Float|Round (.y _numberofinstancesrange)))))
      (for _index (range 0 (- _output_get 1))
        (Components|InstancedStaticMesh|AddInstance (Variables|Default|GetInstancedStaticMesh) (Math|Transform|MakeTransform (+ (* (Math|Vector|GetForwardVector (Math|Rotator|MakeRotator 0.0 0.0 (Math|Random|RandomFloatinRange -1.8e+02 1.8e+02))) (Math|Random|RandomFloatinRange (* _returnvalue -1.0) _returnvalue)) (Transformation|GetActorLocation)) (Math|Rotator|MakeRotator 0.0 0.0 (Math|Random|RandomFloatinRange -1.8e+02 1.8e+02)) (Math|Conversions|ToVector(Float) (Math|Random|RandomFloatinRange (.x _scalerange) (.y _scalerange)))) true)))))