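; BP_SplineMeshArray is an actor that repeats a chosen static mesh at even intervals along a spline.
; The construction script derives spacing from the mesh bounding box's scaled X size plus an offset, then fits the count to the spline length.
; Each copy is an instanced static mesh placed in local space with zero rotation, so copies follow the spline's position but neither turn nor bend with it.
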(event EventBeginPlay)

(fn ConstructionScript
  (bind _mesh (Variables|Config|GetMesh))
  (bind _returnvalue (StaticMesh|GetBoundingBox _mesh))
  (bind (_min _max) (Utilities|Struct|BreakBox _returnvalue))
  (Utilities|IsValid _mesh
    (:Is%20Valid
      (Components|StaticMesh|SetStaticMesh (Variables|Default|GetInstancedStaticMesh) _mesh)
      (bind _output_get (Variables|Default|SetSpacing (+ (.X (Math|Vector|BreakVector (* (- _max _min) (Variables|Config|GetScale)))) (Variables|Config|GetOffset))))
      (bind _output_get_2 (LocalVariables|SetNumberOfInstances (Math|Float|Floor (/ (Spline|GetSplineLength (Variables|Default|GetSpline)) _output_get))))
      (for _index (range 0 _output_get_2)
        (Components|InstancedStaticMesh|AddInstance (Variables|Default|GetInstancedStaticMesh) (Math|Transform|MakeTransform (Spline|GetLocationatDistanceAlongSpline (Variables|Default|GetSpline) (* _index (Variables|Default|GetSpacing)) "Local") "0, 0, 0" (Variables|Config|GetScale)) false)))))