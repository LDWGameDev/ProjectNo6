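; Floor-exit objective actor that opens once every area control in its array is completed, then lets the player open the upgrade selection panel.
; It listens to each area's completion delegate and, when all are done, shows a "Gate Opened" notification and signals floor completion to the game instance.
; Once complete, box overlap shows an "E" prompt and registers it as interactable.
; Pressing E opens the panel and clears the character's floor upgrades.
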(event OnComponentBeginOverlap(Box)
  (params (OverlappedComponent :type Primitive%20Component%20Object%20Reference) (OtherActor :type Actor%20Object%20Reference) (OtherComp :type Primitive%20Component%20Object%20Reference) (OtherBodyIndex :type Integer) (bFromSweep :type Boolean) (SweepResult :type Hit%20Result%20Structure%20%28by%20ref%29))
  ;[1 1 1] Begin Overlap
  (if (CallFunction|IsAllAreasCompleted)
    (bind _asbp_character_player_human (Utilities|Casting|CastToBP_CharacterPlayerHuman OtherActor))
    (Rendering|SetVisibility (Variables|Default|GetWidget) true false)
    (Class|CharacterPlayerBase|AddInteractableActor _asbp_character_player_human self)))

(event OnComponentEndOverlap(Box)
  (params (OverlappedComponent :type Primitive%20Component%20Object%20Reference) (OtherActor :type Actor%20Object%20Reference) (OtherComp :type Primitive%20Component%20Object%20Reference) (OtherBodyIndex :type Integer))
  ;[1 1 1] End Overlap
  (if (CallFunction|IsAllAreasCompleted)
    (bind _asbp_character_player_human (Utilities|Casting|CastToBP_CharacterPlayerHuman OtherActor))
    (Rendering|SetVisibility (Variables|Default|GetWidget) false false)
    (Class|CharacterPlayerBase|RemoveInteractableActor _asbp_character_player_human self)))

(event Custom|HandleOnAreaControlCompletedDelegate
  (params (CompletedAreaControl :type Area%20Control%20Object%20Reference))
  (Utilities|IsValid CompletedAreaControl
    (:Is%20Valid
      (CallFunction|CheckifAllAreaControlAreaCompleted))))

(event EventBeginPlay
  ;[1 1 1] BeginPlay
  (bind _aswbp_interaction_text (Utilities|Casting|CastToWBP_InteractionText (UserInterface|GetWidget (Variables|Default|GetWidget))))
  (Variables|/Game/LDW/Blueprints/Widgets/WBP_InteractionText.WBP_InteractionText_C|SetButtonText _aswbp_interaction_text "E")
  (for _array_element (Variables|Default|GetAreaControlsArray)
    (Utilities|IsValid _array_element
      (:Is%20Valid
        (EventDispatchers|AssignOnAreaControlCompletedDelegate _array_element (delegate Custom|HandleOnAreaControlCompletedDelegate))))))

(fn ConstructionScript)

(fn IsAllAreasCompleted
  (for _array_element (Variables|Default|GetAreaControlsArray)
    (Utilities|IsValid _array_element
      (:Is%20Valid
        (if (not (Variables|/Script/ProjectNo6.AreaControl|GetbIsCompleted _array_element))
          (return false)))
      (:Is%20Not%20Valid
        (return false))))
  (return true))

(fn CheckifAllAreaControlAreaCompleted
  (for _array_element (Variables|Default|GetAreaControlsArray)
    (Utilities|IsValid _array_element
      (:Is%20Valid
        (if (not (Variables|/Script/ProjectNo6.AreaControl|GetbIsCompleted _array_element))
          (LocalVariables|SetAreAllCompleted false)))))
  (if (LocalVariables|GetAreAllCompleted)
    (bind _asbp_player_controller_gameplay (Utilities|Casting|CastToBP_PlayerControllerGameplay (Game|GetPlayerController 0)))
    (Default|Notify (Variables|/Game/LDW/Blueprints/Characters/Player/BP_PlayerControllerGameplay.BP_PlayerControllerGameplay_C|GetPersistentGameplayWBP _asbp_player_controller_gameplay) "Gate Opened")
    (bind _asbp_game_instance_custom (Utilities|Casting|CastToBP_GameInstanceCustom (Game|GetGameInstance)))
    (Default|CallOnCompletedFloor _asbp_game_instance_custom)))

(fn TriggerInteractionKey
  (params (PlayerControllerDoTrigger :type Player%20Controller%20Object%20Reference) (Key :type Key%20Structure%20%28by%20ref%29))
  (if (and (== Key "E") (CallFunction|IsAllAreasCompleted))
    (Utilities|Casting|CastToBP_GameInstanceCustom (Game|GetGameInstance)
      (:then
        (bind _asbp_player_controller_gameplay (Utilities|Casting|CastToBP_PlayerControllerGameplay (Game|GetPlayerController 0))
          (:then
            (Default|SetState (Variables|/Game/LDW/Blueprints/Characters/Player/BP_PlayerControllerGameplay.BP_PlayerControllerGameplay_C|GetUpgradeSelectionsPanel _asbp_player_controller_gameplay) true)
            (Default|ClearFloorUpgradesArray (.AsBP%20Character%20Player%20Human (Utilities|Casting|CastToBP_CharacterPlayerHuman (Pawn|GetControlledPawn _asbp_player_controller_gameplay))))
            (return true))
          (:CastFailed
            _)))
      (:CastFailed
        _)))
  (return false))