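; BP_TriggerTempleSelection is an interactable trigger that lets the human player start temple selection with the E key.
; Its box overlap shows or hides the key prompt and registers the actor with the character as interactable.
; An indicator widget starts active and is switched off permanently on the first player overlap.
; TriggerInteractionKey generates floor objectives in the game instance, calls temple selection on the player controller and plays a sound.
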(event OnComponentBeginOverlap(Box)
  (params (OverlappedComponent :type Primitive%20Component%20Object%20Reference) (OtherActor :type Actor%20Object%20Reference) (OtherComp :type Primitive%20Component%20Object%20Reference) (OtherBodyIndex :type Integer) (bFromSweep :type Boolean) (SweepResult :type Hit%20Result%20Structure%20%28by%20ref%29))
  ;[1 1 1] Begin Overlap
  (bind _asbp_character_player_human (Utilities|Casting|CastToBP_CharacterPlayerHuman OtherActor))
  (Rendering|SetVisibility (Variables|Default|GetInteraction%20Input) true false)
  (Class|CharacterPlayerBase|AddInteractableActor _asbp_character_player_human self)
  (if (not (Variables|Default|GetbHasDisableInteractableIndicator))
    (bind _interactableindicatorwidget (Utilities|GetInteractableIndicatorWidget)
      (:Valid
        (Default|SetState _interactableindicatorwidget false)
        (Variables|Default|SetbHasDisableInteractableIndicator true)))))

(event OnComponentEndOverlap(Box)
  (params (OverlappedComponent :type Primitive%20Component%20Object%20Reference) (OtherActor :type Actor%20Object%20Reference) (OtherComp :type Primitive%20Component%20Object%20Reference) (OtherBodyIndex :type Integer))
  ;[1 1 1] End Overlap
  (bind _asbp_character_player_human (Utilities|Casting|CastToBP_CharacterPlayerHuman OtherActor))
  (Rendering|SetVisibility (Variables|Default|GetInteraction%20Input) false false)
  (Class|CharacterPlayerBase|RemoveInteractableActor _asbp_character_player_human self))

(event EventBeginPlay
  ;[1 1 1] BeginPlay
  (bind _aswbp_interaction_text (Utilities|Casting|CastToWBP_InteractionText (UserInterface|GetWidget (Variables|Default|GetInteraction%20Input))))
  (Variables|/Game/LDW/Blueprints/Widgets/WBP_InteractionText.WBP_InteractionText_C|SetButtonText _aswbp_interaction_text "E")
  (bind _interactableindicatorwidget (Utilities|GetInteractableIndicatorWidget)
    (:Valid
      (Default|SetState _interactableindicatorwidget true))))

(fn ConstructionScript)

(fn TriggerInteractionKey
  (params (PlayerControllerDoTrigger :type Player%20Controller%20Object%20Reference) (Key :type Key%20Structure%20%28by%20ref%29 :default "None"))
  (bind _returnvalue (== Key "E"))
  (bind _asbp_player_controller_gameplay (Utilities|Casting|CastToBP_PlayerControllerGameplay PlayerControllerDoTrigger)
    (:then
      (if _returnvalue
        (bind _asbp_game_instance_custom (Utilities|Casting|CastToBP_GameInstanceCustom (Game|GetGameInstance))
          (:then
            (Class|GameInstanceCustom|GenerateFloorObjectives _asbp_game_instance_custom)
            (Class|PlayerControllerGameplay|TriggerTempleSelection _asbp_player_controller_gameplay)
            (Audio|SpawnSound2D "/Game/LDW/Assets/Sounds/S_Special_1.S_Special_1" 1.0 1.0 0.0 0)
            (return _returnvalue))
          (:CastFailed
            _))))
    (:CastFailed
      _))
  (return false))