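; BP_TimerBomb is a trap actor that starts a short fuse when activated, including when it takes damage, then explodes.
; It builds on a parent trap class, binding its Combat component's damage delegate to trap activation.
; Activation lights the mesh's Lava material parameter, shows Niagara effects and plays ticking audio.
; After a delay, it deals random damage to sphere-overlapped actors, spawns explosion sound, particles and camera shake, and destroys itself.
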(event Custom|HandleOnTookDamage
  (params (DamageDetailsTaken :type Damage%20Details%20Object%20Reference))
  (Class|TrapBase|ActivateTrap))

(event EventBeginPlay
  (|CallParentFunction)
  (EventDispatchers|AssignOnTookDamageDelegate (Variables|Default|GetCombat) (delegate Custom|HandleOnTookDamage)))

(event EventOnTrapActivated
  (|CallParentFunction)
  (Utilities|FlowControl|Sequence
    (:then_0
      (Rendering|Material|SetScalarParameterValueonMaterials (Variables|Default|GetBombMesh) "Lava" 1.0)
      (Rendering|SetVisibility (Variables|Default|GetNiagara) true false)
      (Audio|SpawnSoundatLocation "/Game/LDW/Assets/Sounds/S_TimerBombTick_Cue.S_TimerBombTick_Cue" (Transformation|GetActorLocation) "0, 0, 0" 1.0 1.0 0.0 0 0))
    (:then_1
      (Utilities|FlowControl|Delay 1.5)
      (Rendering|SetVisibility (Variables|Default|GetNiagara) false false)
      (Utilities|FlowControl|Sequence
        (:then_0
          (bind _outactors (Collision|SphereOverlapActors (Transformation|GetActorLocation) 4.5e+02 (Utilities|Array|MakeArray "ObjectTypeQuery3" "ObjectTypeQuery8") "/Script/Engine.Actor" (Utilities|Array|MakeArray 0)))
          (for _array_element _outactors
            (CallFunction|CreateandDealDamage _array_element (Math|Random|RandomIntegerinRange 18 20)))
          (Utilities|FlowControl|Delay 0.0)
          (Actor|DestroyActor))
        (:then_1
          (Audio|SpawnSoundatLocation "/Game/LDW/Assets/Sounds/S_TimerBombExplosion_Cue.S_TimerBombExplosion_Cue" (Transformation|GetActorLocation) "0, 0, 0" 1.0 1.0 0.0 0 0)
          (Effects|SpawnEmitteratLocation "/Game/AdvancedMagicFX05/Particles/P_AMFX05_spark2.P_AMFX05_spark2" (Transformation|GetActorLocation) "0, 0, 0" "2.500000,2.500000,2.500000")
          (Camera|PlayWorldCameraShake "/Game/LDW/Blueprints/Data/CameraShake/CS_MediumShake.CS_MediumShake_C" (Transformation|GetActorLocation) 3e+03 5e+03))))))

(event EventDeactivateTrap
  (|CallParentFunction))

(fn ConstructionScript
  (|CallParentFunction))