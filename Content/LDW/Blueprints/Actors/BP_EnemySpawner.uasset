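; Enemy spawner Blueprint that adds a ground indicator effect whenever it spawns an enemy.
; SpawnEnemy overrides the parent, calls its spawn logic, passes the result to SpawnFXIndicatorAtEnemyFoot and returns that enemy.
; For a valid enemy, the helper spawns the NS_EnemySpawnIndicator system just above its feet, derived from actor location and scaled capsule half-height.
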(event EventBeginPlay)

(fn ConstructionScript)

(fn SpawnEnemy
  (bind _returnvalue (|CallParentFunction))
  (CallFunction|SpawnFXIndicatoratEnemyFoot _returnvalue)
  (return _returnvalue))

(fn SpawnFXIndicatoratEnemyFoot
  (params (Enemy :type Character%20Enemy%20Base%20Object%20Reference))
  (Utilities|IsValid Enemy
    (:Is%20Valid
      (Niagara|SpawnSystematLocation "/Game/AdvancedMagicFX16/Particles/Niagara/NS_EnemySpawnIndicator.NS_EnemySpawnIndicator" (+ (Transformation|GetActorLocation Enemy) "" "0,0,10.000000" (Math|Vector|MakeVector 0.0 0.0 (* (Components|Capsule|GetScaledCapsuleHalfHeight (Variables|/Script/Engine.Character|GetCapsuleComponent Enemy)) -1.0)))))))