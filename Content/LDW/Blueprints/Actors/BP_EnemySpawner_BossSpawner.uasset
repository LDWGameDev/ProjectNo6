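; Enemy spawner variant, named for boss use, that periodically spawns and activates enemies while keeping a small cap on how many exist.
; After an initial delay, a looping timer prunes invalid references before spawning more.
; Overrides of parent functions randomize locations within a navigable radius and play a Niagara indicator at each enemy's feet.
; A cleanup event stops the timer and force-kills all tracked enemies.
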(event Custom|SpawnEnemyWithAmountCheck
  (bind _returnvalue (CallFunction|CheckSpawnedEnemies))
  (if (< _returnvalue 3)
    (bind _returnvalue_2 (CallFunction|SpawnEnemy))
    (bind _asbp_enemy_base (Utilities|Casting|CastToBP_EnemyBase _returnvalue_2))
    (Default|TryActivateEnemy _asbp_enemy_base)
    (Utilities|Array|Add (Variables|Default|GetSpawnedEnemies) _asbp_enemy_base)))

(event Custom|StartSpawningPeriodically
  (Utilities|FlowControl|Delay 6.0)
  (bind _returnvalue (Utilities|Time|SetTimerbyEvent (delegate Custom|SpawnEnemyWithAmountCheck) 15.0 true))
  (Variables|Default|SetSpawnOverTimeTimerHandle _returnvalue))

(event Custom|DestroyAllSpawnedEnemies
  (bind _spawnedenemies (Variables|Default|GetSpawnedEnemies))
  (Utilities|Time|ClearandInvalidateTimerbyHandle (Variables|Default|GetSpawnOverTimeTimerHandle))
  (for _array_element _spawnedenemies
    (Class|CharacterEnemyBase|ForceonDied _array_element))
  (Utilities|Array|Clear _spawnedenemies))

(event EventBeginPlay)

(fn ConstructionScript)

(fn SpawnEnemy
  (bind _returnvalue (|CallParentFunction))
  (CallFunction|SpawnFXIndicatoratEnemyFoot _returnvalue)
  (return _returnvalue))

(fn SpawnFXIndicatoratEnemyFoot
  (params (Enemy :type Character%20Enemy%20Base%20Object%20Reference))
  (Utilities|IsValid Enemy
    (:Is%20Valid
      (Niagara|SpawnSystematLocation "/Game/AdvancedMagicFX16/Particles/Niagara/NS_EnemySpawnIndicator.NS_EnemySpawnIndicator" (+ (Transformation|GetActorLocation Enemy) "" "0,0,10.000000" (Math|Vector|MakeVector 0.0 0.0 (* (Components|Capsule|GetScaledCapsuleHalfHeight (Variables|/Script/Engine.Character|GetCapsuleComponent Enemy)) -1.0)))))))

(fn CheckSpawnedEnemies
  (bind _tempenemiesarray (LocalVariables|GetTempEnemiesArray))
  (for _array_element (Variables|Default|GetSpawnedEnemies)
    (Utilities|IsValid _array_element
      (:Is%20Valid
        (Utilities|Array|Add (LocalVariables|GetTempEnemiesArray) _array_element))))
  (Variables|Default|SetSpawnedEnemies _tempenemiesarray)
  (return (Utilities|Array|Length _tempenemiesarray)))

(fn GetSpawnLocation
  (bind _returnvalue (|CallParentFunction))
  (bind (_randomlocation _returnvalue_2) (Class|NavigationSystemV1|GetRandomLocationinNavigableRadius _returnvalue 1.2e+03 0 0))
  (if _returnvalue_2
    (return _randomlocation)
    (else
      (return _returnvalue))))