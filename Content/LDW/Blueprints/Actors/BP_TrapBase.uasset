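; BP_TrapBase is a base Blueprint for traps that activate and deal damage.
; ActivateTrap runs the parent implementation and, only on success, fires the OnTrapActivated event, which is empty here.
; CreateAndDealDamage builds a DamageDetails object with the trap as instigator and passes it to the target's CombatComponent, if one exists.
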(event Custom|OnTrapActivated)

(fn ConstructionScript)

(fn ActivateTrap
  (bind _returnvalue (|CallParentFunction))
  (if _returnvalue
    (CallFunction|OnTrapActivated)
    (return true)
    (else
      (return false))))

(fn CreateandDealDamage
  (params (TargetTakeDamage :type Actor%20Object%20Reference) (Damage :type Integer))
  (bind _returnvalue (Actor|GetComponentbyClass TargetTakeDamage "/Script/ProjectNo6.CombatComponent"))
  (bind _returnvalue_2 (Game|ConstructObjectfromClass "/Script/ProjectNo6.DamageDetails"))
  (Variables|/Script/ProjectNo6.DamageDetails|SetDamage _returnvalue_2 Damage)
  (Variables|/Script/ProjectNo6.DamageDetails|SetTargetActor _returnvalue_2 TargetTakeDamage)
  (Variables|/Script/ProjectNo6.DamageDetails|SetInstigatorActor _returnvalue_2 self)
  (Utilities|IsValid _returnvalue
    (:Is%20Valid
      (Class|CombatComponent|TakeDamage _returnvalue _returnvalue_2))))