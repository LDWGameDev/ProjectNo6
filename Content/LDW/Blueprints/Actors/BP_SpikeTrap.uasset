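; Spike trap actor that damages whatever stands in its Box trigger, built on a parent trap class that supplies activation and cooldown state.
; A human player or enemy entering the box plays a warning sound and, after a short delay, calls ActivateTrap.
; OnTrapActivated moves the spikes, deals one randomized hit to every overlapping actor regardless of type, then deactivates after a few seconds, resetting the spikes.
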(event OnComponentBeginOverlap(Box)
  (params (OverlappedComponent :type Primitive%20Component%20Object%20Reference) (OtherActor :type Actor%20Object%20Reference) (OtherComp :type Primitive%20Component%20Object%20Reference) (OtherBodyIndex :type Integer) (bFromSweep :type Boolean) (SweepResult :type Hit%20Result%20Structure%20%28by%20ref%29))
  (if (Math|Boolean|ANDBoolean (or (.bSuccess (Utilities|Casting|CastToBP_CharacterPlayerHuman OtherActor)) (.bSuccess (Utilities|Casting|CastToBP_EnemyBase OtherActor))) (not (Variables|Default|GetbHasDelayActivateTrap)) (not (Variables|Default|GetbIsInCooldown)) (not (Variables|Default|GetbIsActivated)))
    (Variables|Default|SetbHasDelayActivateTrap true)
    (Audio|PlaySoundatLocation "/Game/LDW/Assets/Sounds/S_TrapActivate_01_Cue.S_TrapActivate_01_Cue" (Transformation|GetActorLocation) "0, 0, 0" 1.0 1.0 0.0 0 0 0 0)
    (Utilities|FlowControl|Delay 0.7)
    (Class|TrapBase|ActivateTrap)))

(event EventBeginPlay
  (|CallParentFunction))

(event EventOnTrapActivated
  (Utilities|FlowControl|Sequence
    (:then_0
      (Transformation|SetRelativeLocation (Variables|Default|GetTrapSpikes) "0, 0,3.000000" false false)
      (Variables|Default|SetbHasDelayActivateTrap false)
      (Audio|PlaySoundatLocation "/Game/LDW/Assets/Sounds/S_SpikeTrapRaiseUp_Cue.S_SpikeTrapRaiseUp_Cue" (Transformation|GetActorLocation) "0, 0, 0" 1.0 1.0 0.0 0 0 0 0)
      (for _array_element (Collision|GetOverlappingActors (Variables|Default|GetBox) "/Script/Engine.Actor" :!class /Script/Engine.PrimitiveComponent)
        (CallFunction|CreateandDealDamage _array_element (Math|Random|RandomIntegerinRange 14 16))))
    (:then_1
      (Utilities|FlowControl|Delay 3.0)
      (Class|TrapBase|DeactivateTrap))))

(event EventDeactivateTrap
  (|CallParentFunction)
  (Transformation|SetRelativeLocation (Variables|Default|GetTrapSpikes) "0, 0,16.000000" false false))

(fn ConstructionScript
  (|CallParentFunction))