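; Fire statue trap that activates when a human player character or enemy enters its box, then burns nearby actors.
; Activation shows a Niagara effect with sound, then after a short delay reveals the firestorm, damaging immediately and on a looping timer through a sphere overlap with random damage.
; After a few seconds, a timeline rescales the firestorm, then deactivates the trap, hiding both effects and clearing the timer.
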(event OnComponentBeginOverlap(Box)
  (params (OverlappedComponent :type Primitive%20Component%20Object%20Reference) (OtherActor :type Actor%20Object%20Reference) (OtherComp :type Primitive%20Component%20Object%20Reference) (OtherBodyIndex :type Integer) (bFromSweep :type Boolean) (SweepResult :type Hit%20Result%20Structure%20%28by%20ref%29))
  (if (or (.bSuccess (Utilities|Casting|CastToBP_CharacterPlayerHuman OtherActor)) (.bSuccess (Utilities|Casting|CastToBP_EnemyBase OtherActor)))
    (Class|TrapBase|ActivateTrap)))

(event Custom|DealDamage
  (bind _outactors (Collision|SphereOverlapActors (Transformation|GetWorldLocation (Variables|Default|GetNiagara)) 265.0 (Utilities|Array|MakeArray "ObjectTypeQuery3" "ObjectTypeQuery8") "/Script/Engine.Actor" (Utilities|Array|MakeArray 0)))
  (for _array_element _outactors
    (CallFunction|CreateandDealDamage _array_element (Math|Random|RandomIntegerinRange 5 7))))

(event EventOnTrapActivated
  (bind _p_ky_firestorm (Variables|Default|GetP_ky_fireStorm))
  (|CallParentFunction)
  (Utilities|FlowControl|Sequence
    (:then_0
      (Rendering|SetVisibility (Variables|Default|GetNiagara) true false)
      (Audio|SpawnSoundatLocation "/Game/LDW/Assets/Sounds/Fire_Spelll_37_Cue.Fire_Spelll_37_Cue" (Transformation|GetActorLocation) "0, 0, 0" 1.0 1.0 0.0 0 0))
    (:then_1
      (Utilities|FlowControl|Delay 1.2)
      (Utilities|FlowControl|Sequence
        (:then_0
          (Rendering|SetVisibility _p_ky_firestorm true false)
          (Transformation|SetWorldScale3D _p_ky_firestorm "1.000000,1.000000,1.000000")
          (bind _returnvalue (Utilities|Time|SetTimerbyEvent (delegate Custom|DealDamage) 0.75 true))
          (Variables|Default|SetDealDamageTimerHandle _returnvalue)
          (bind _outactors (Collision|SphereOverlapActors (Transformation|GetWorldLocation (Variables|Default|GetNiagara)) 265.0 (Utilities|Array|MakeArray "ObjectTypeQuery3" "ObjectTypeQuery8") "/Script/Engine.Actor" (Utilities|Array|MakeArray 0)))
          (for _array_element _outactors
            (CallFunction|CreateandDealDamage _array_element (Math|Random|RandomIntegerinRange 5 7))))
        (:then_1
          (Utilities|FlowControl|Delay 4.5)
          (bind _newtrack_0 (Timeline|SmallerFlame PlayFromStart)
            (:Update
              (Transformation|SetWorldScale3D (Variables|Default|GetP_ky_fireStorm) (Math|Conversions|ToVector(Float) _newtrack_0)))
            (:Finished
              (Class|TrapBase|DeactivateTrap))))))))

(event EventDeactivateTrap
  (|CallParentFunction)
  (Rendering|SetVisibility (Variables|Default|GetNiagara) false false)
  (Rendering|SetVisibility (Variables|Default|GetP_ky_fireStorm) false false)
  (Utilities|Time|ClearandInvalidateTimerbyHandle (Variables|Default|GetDealDamageTimerHandle)))

(fn ConstructionScript
  (|CallParentFunction))