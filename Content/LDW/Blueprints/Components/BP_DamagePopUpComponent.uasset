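; BP_DamagePopUpComponent is a component that shows damage numbers on its owner through a pool of screen-space WBP_DamagePopUp widgets.
; On BeginPlay it adds a configurable number of widget components to the owner, each holding its own pop-up widget.
; PopUpDamage passes the value to a pooled widget chosen by a wrapping index.
; GetNextIndex advances that index on every call, including separately for the validity check and widget lookup.
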(event EventBeginPlay
  (bind _returnvalue (Components|GetOwner))
  (Utilities|IsValid _returnvalue
    (:Is%20Valid
      (for _index (range 0 (- (Variables|Config|GetNumberOfDamageComponents) 1))
        (bind _returnvalue_2 (Game|AddComponentbyClass _returnvalue "/Script/UMG.WidgetComponent" false (Math|Transform|MakeTransform (Variables|Config|GetRelativeLocation) "0, 0, 0" "1.000000,1.000000,1.000000")))
        (Utilities|FlowControl|Sequence
          (:then_0
            (bind _returnvalue_3 (Game|ConstructObjectfromClass self "/Game/LDW/Blueprints/Widgets/WBP_DamagePopUp.WBP_DamagePopUp_C"))
            (UserInterface|SetWidget _returnvalue_2 _returnvalue_3))
          (:then_1
            (Class|WidgetComponent|SetWidgetSpace _returnvalue_2 "Screen")
            (Class|WidgetComponent|SetDrawatDesiredSize _returnvalue_2 true))
          (:then_2
            (Utilities|Array|Add (Variables|Default|GetDamageWidgetComps) _returnvalue_2)))))))

(fn GetNextIndex
  (if (>= (+ (Variables|Default|GetCurrentIndex) 1) (Variables|Config|GetNumberOfDamageComponents))
    (Variables|Default|SetCurrentIndex 0)
    (else
      (Variables|Default|SetCurrentIndex (+ (Variables|Default|GetCurrentIndex) 1))))
  (return (Variables|Default|GetCurrentIndex)))

(fn PopUpDamage
  (params (DamageValue :type Integer))
  (bind _nextindex (CallFunction|GetNextIndex))
  (bind _damagewidgetcomps (Variables|Default|GetDamageWidgetComps))
  (bind _output (Utilities|Array|Get(acopy) _damagewidgetcomps _nextindex))
  (Utilities|IsValid _output
    (:Is%20Valid
      (bind _aswbp_damage_pop_up (Utilities|Casting|CastToWBP_DamagePopUp (UserInterface|GetWidget _output)))
      (Default|SetDamageValueandShowUp _aswbp_damage_pop_up DamageValue))))