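; Shooting star effect actor for the AdvancedMagicFX16 pack that moves a Niagara component along a scripted arc and then removes itself.
; On BeginPlay a timeline drives per-frame relative offsets, scaling its X, Y and Z curves by shot length, lateral and height variables and delta time.
; Delays chained off the timeline update zero the effect's relative Z to correct its landing, then destroy the actor a second later.
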(event EventBeginPlay
  (bind _niagara (Variables|Default|GetNiagara))
  (bind _relativelocation (Variables|/Script/Engine.SceneComponent|GetRelativeLocation _niagara))
  ;[1 1 1] effect move control
  (bind (_direction _x _y _z) (Timeline|Timeline_0 PlayFromStart)
    (:Update
      (Transformation|AddRelativeLocation (Variables|Default|GetNiagara) (Math|Vector|MakeVector (* (* (Variables|Default|GetshotLength) _x) (stale EventTick DeltaSeconds)) (* (stale EventTick DeltaSeconds) (* (Variables|Default|GetshotY) _y)) (* (stale EventTick DeltaSeconds) (* (Variables|Default|GetshotHight) _z))) false false)
      ;[1 1 1] location correct
      (Utilities|FlowControl|Delay 0.41)
      (Transformation|SetRelativeLocation _niagara (Math|Vector|MakeVector (.x _relativelocation) (.y _relativelocation) 0.0) false false)
      ;[1 1 1] effect destroy
      (Utilities|FlowControl|Delay 1.0)
      (Actor|DestroyActor))))

(event Collision|EventActorBeginOverlap
  (params (OtherActor :type Actor%20Object%20Reference)))

(event EventTick
  (params (DeltaSeconds :type Float%20%28single-precision%29))
  ;[1 1 1] effect move control
)

(fn ConstructionScript)